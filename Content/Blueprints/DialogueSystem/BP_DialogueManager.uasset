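; Dialogue manager that plays timed conversations in a WBP_DialogueUI widget, with per-sentence text, image and 2D sound.
; StartDialogue ignores calls while running; StartMonologue sets the speaker name and loads each part's sentences into parallel queue arrays behind a blank placeholder.
; DisplayNextSentence pops the front, then auto-advances after a delay indexed by monologue, not queue front.
; After the last part, EndDialogue removes the widget and hides the cursor.
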(event `DisplaySentence`
  (bind _output_get (set `self.NewVar` (`|GetArrayItem` (`self.CurrentTmer`) (`self.CurrentMonologueIndex`))))
  (`KismetSystemLibrary.Delay` _output_get)
  (`self.DisplayNextSentence`))

(event `self.ReceiveBeginPlay`
  (bind _returnvalue (`|CreateWidget` "/Game/Blueprints/DialogueSystem/WBP_DialogueUI.WBP_DialogueUI_C"))
  (set `self.DIalogueUI` _returnvalue))

(fn `AddToCurrent`
  (params (Text :type "String (by ref)") (Timer :type "Float (double-precision) (by ref)") (Image :type "Texture2D Object Reference (by ref)") (Audio :type "SoundWave Object Reference (by ref)"))
  (`KismetArrayLibrary.Array_Add` (`self.CurrentText`) Text)
  (`KismetArrayLibrary.Array_Add` (`self.CurrentTmer`) Timer)
  (`KismetArrayLibrary.Array_Add` (`self.CurrentImage`) Image)
  (`KismetArrayLibrary.Array_Add` (`self.CurrentAudio`) Audio)
  (return))

(fn `DisplayNextSentence`
  (locals (Sentence :type String))
  (`self.RemoveFromCurrent`)
  (if (== (`KismetArrayLibrary.Array_Length` (`self.CurrentText`)) 0)
    (if (< (`self.CurrentMonologueIndex`) (- (`KismetArrayLibrary.Array_Length` (`.DialogueParts_3_8AD1EFBE4AE101803C8A23B464C81367` (break `/Game/Blueprints/DialogueSystem/S_Dialogue` (`self.ActualDialogue`)))) 1))
      (set `self.CurrentMonologueIndex` (+ (`self.CurrentMonologueIndex`) 1))
      (`self.StartMonologue`)
      (bind (_text _timer _image _audio) (`self.GetFromCurrent` :!label _label))
      (`self.TypeSentence` _text _image _audio)
      (`self.DisplaySentence`)
      (else
        (`self.EndDialogue`)))
    (else
      (goto _label))))

(fn `EndDialogue`
  (locals (`Empty DIalogue` :type "/Game/Blueprints/DialogueSystem/S_Dialogue Structure"))
  (set `self.ActualDialogue` (`local.Empty DIalogue`))
  (set `self.CurrentMonologueIndex` 0)
  (`Widget.RemoveFromParent` (`self.DIalogueUI`))
  (set `PlayerController.bShowMouseCursor` false (`GameplayStatics.GetPlayerController` 0))
  (set `self.IsRunning` false))

(fn `GetFromCurrent`
  (returns (Text :type "String (by ref)") (Timer :type "Float (double-precision) (by ref)") (Image :type "Texture2D Object Reference") (Audio :type "SoundWave Object Reference"))
  (return (`|GetArrayItem` (`self.CurrentText`)) (`|GetArrayItem` (`self.CurrentTmer`)) (`|GetArrayItem` (`self.CurrentImage`)) (`|GetArrayItem` (`self.CurrentAudio`))))

(fn `RemoveFromCurrent`
  (`KismetArrayLibrary.Array_Remove` (`self.CurrentText`))
  (`KismetArrayLibrary.Array_Remove` (`self.CurrentTmer`))
  (`KismetArrayLibrary.Array_Remove` (`self.CurrentImage`))
  (`KismetArrayLibrary.Array_Remove` (`self.CurrentAudio`))
  (return))

(fn `StartDialogue`
  (params (indexDialogue :type "/Game/Blueprints/DialogueSystem/S_Dialogue Structure"))
  (if (not (`self.IsRunning`))
    (set `self.IsRunning` true)
    (`UserWidget.AddToViewport` (`self.DIalogueUI`) 0)
    (set `self.ActualDialogue` indexDialogue)
    (`self.StartMonologue`)
    (return)))

(fn `StartMonologue`
  (locals (Empty :type String) (`Empty Current Text` :type "Array of String") (`Empty Current Timer` :type "Array of Float (double-precision)") (`Empty Current Image` :type "Array of Texture2D Object Reference"))
  (bind (_name _sentences) (break `/Game/Blueprints/DialogueSystem/S_Monologue` (`|GetArrayItem` (`.DialogueParts_3_8AD1EFBE4AE101803C8A23B464C81367` (break `/Game/Blueprints/DialogueSystem/S_Dialogue` (`self.ActualDialogue`))) (`self.CurrentMonologueIndex`))))
  (set `/Game/Blueprints/DialogueSystem/WBP_DialogueUI.Name` (`KismetTextLibrary.Conv_StringToText` _name) (`self.DIalogueUI`))
  (set `self.CurrentText` (`local.Empty Current Text`))
  (set `self.CurrentTmer` (`local.Empty Current Timer`))
  (set `self.CurrentImage` (`local.Empty Current Image`))
  (`self.AddToCurrent` "")
  (for _array_element _sentences
    (bind (_sentence _timer _audioclip _image) (break `/Game/Blueprints/DialogueSystem/S_Sentence` _array_element))
    (`self.AddToCurrent` _sentence _timer _image _audioclip))
  (`self.DisplayNextSentence`))

(fn `TypeSentence`
  (params (InString :type String) (Image :type "Texture2D Object Reference") (Audio :type "SoundWave Object Reference"))
  (bind _dialogueui (`self.DIalogueUI`))
  (set `/Game/Blueprints/DialogueSystem/WBP_DialogueUI.Sentence` (`KismetTextLibrary.Conv_StringToText` InString) _dialogueui)
  (set `/Game/Blueprints/DialogueSystem/WBP_DialogueUI.Image` Image _dialogueui)
  (`GameplayStatics.PlaySound2D` Audio 1.0 1.0 0.0 null null))

(fn `UserConstructionScript`)