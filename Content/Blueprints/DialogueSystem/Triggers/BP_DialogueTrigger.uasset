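; BP_DialogueTrigger is a placeable trigger that starts its assigned dialogue through the DialogueManager.
; It fires when BP_Player overlaps its Box or through the TrigDialogue event, which is bound to an OnDialogueTrig event on BeginPlay.
; After firing, the Retrigger macro disables the Box's overlap events, restoring them after a delay only if the trigger is retriggerable.
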(event `self.ReceiveBeginPlay`
  (add `self.OnDialogueTrig` (delegate `TrigDialogue`)))

(event `TrigDialogue`
  (`self.TriggerDialogue` (`self.MyDialogue`) :!label _label)
  (`self.Retrigger` (`self.Box`) (`self.Delay`) (`self.isRetriggerable`)))

(event `self.Box.OnComponentBeginOverlap`
  (params (OverlappedComponent :type "PrimitiveComponent Object Reference") (OtherActor :type "Actor Object Reference") (OtherComp :type "PrimitiveComponent Object Reference") (OtherBodyIndex :type Integer) (bFromSweep :type Boolean) (SweepResult :type "HitResult Structure (by ref)"))
  (cast `/Game/Blueprints/Player/BP_Player` OtherActor)
  (goto _label))

(fn `TriggerDialogue`
  (params (indexDialogue :type "/Game/Blueprints/DialogueSystem/S_Dialogue Structure"))
  (`/Game/Blueprints/DialogueSystem/BP_DialogueManager.StartDialogue` (`self.DialogueManager`) indexDialogue))

(fn `UserConstructionScript`)