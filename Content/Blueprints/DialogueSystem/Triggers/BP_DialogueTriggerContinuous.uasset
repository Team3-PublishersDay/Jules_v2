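; Dialogue trigger volume that plays its dialogue repeatedly when its box is overlapped.
; BeginPlay sums every sentence timer into the interval between plays.
; A delayed-loop macro fires the dialogue from index zero through AmountOfTimes inclusive, waiting that interval after each play.
; On completion, the box's overlap events are switched off, then restored after a separate delay if retriggerable.
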(event `self.ReceiveBeginPlay`
  (for _array_element (`.DialogueParts_3_8AD1EFBE4AE101803C8A23B464C81367` (break `/Game/Blueprints/DialogueSystem/S_Dialogue` (`self.MyDialogue`)))
    (for _array_element_2 (`.Sentences_10_904C7D1C4A31FB63A36A8CA63BD4F36F` (break `/Game/Blueprints/DialogueSystem/S_Monologue` _array_element))
      (set `self.ContinuousDelay` (+ (`.Timer_5_6D3CD1504750097B42B7A8A41E622C04` (break `/Game/Blueprints/DialogueSystem/S_Sentence` _array_element_2)) (`self.ContinuousDelay`))))))

(event `self.Box.OnComponentBeginOverlap`
  (params (OverlappedComponent :type "PrimitiveComponent Object Reference") (OtherActor :type "Actor Object Reference") (OtherComp :type "PrimitiveComponent Object Reference") (OtherBodyIndex :type Integer) (bFromSweep :type Boolean) (SweepResult :type "HitResult Structure (by ref)"))
  (`self.For Loop Delay` 0 (`self.AmountOfTimes`) (`self.ContinuousDelay`)
    (:`Loop Body`
      (`self.TriggerDialogue` (`self.MyDialogue`)))
    (:`Completed`
      (`self.Retrigger` (`self.Box`) (`self.Delay`) (`self.isRetriggerable`)))))

(fn `UserConstructionScript`
  (`parent.UserConstructionScript`))