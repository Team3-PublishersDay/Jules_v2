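; Box trigger that starts a random dialogue when something overlaps it.
; The overlap picks a random entry from DialoguePool and passes it to the DialogueManager's StartDialogue.
; Retrigger then switches off the box's overlap events, restoring them after a delay if the trigger is retriggerable and leaving them off otherwise, so it fires only once.
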(event `self.Box.OnComponentBeginOverlap`
  (params (OverlappedComponent :type "PrimitiveComponent Object Reference") (OtherActor :type "Actor Object Reference") (OtherComp :type "PrimitiveComponent Object Reference") (OtherBodyIndex :type Integer) (bFromSweep :type Boolean) (SweepResult :type "HitResult Structure (by ref)"))
  (`self.DialogueTrigger`)
  (`self.Retrigger` (`self.Box`) (`self.Delay`) (`self.isRetriggerable`)))

(fn `DialogueTrigger`
  (`/Game/Blueprints/DialogueSystem/BP_DialogueManager.StartDialogue` (`self.DialogueManager`) (`|GetArrayItem` (`self.DialoguePool`) (`KismetMathLibrary.RandomInteger` (`KismetArrayLibrary.Array_Length` (`self.DialoguePool`))))))

(fn `UserConstructionScript`
  (`parent.UserConstructionScript`))