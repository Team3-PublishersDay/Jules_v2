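; BPC_DamageSystem is a component that tracks health, damage, death and delayed health regeneration for its owner.
; TakeDamage ignores hits when dead, otherwise cancels regeneration, subtracts health, then either calls death or reports the damage response and restarts regeneration.
; A looping timer with an initial delay adds health each tick, broadcasting the value before clamping to MaxHealth and stopping.
; ResetHP restores full health and clears the dead flag.
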(event `RegainingHealt`
  (`self.Heal`))

(fn `Heal`
  (bind _output_get (set `self.Health` (+ (`self.Health`) (* (`self.HealtGeneratedPerSecond`) (`self.RegainingHPForSeconds`)))))
  (`self.OnRegainignHealt` _output_get)
  (if (>= (`self.Health`) (`self.MaxHealth`))
    (set `self.Health` (`self.MaxHealth`))
    (`KismetSystemLibrary.K2_ClearAndInvalidateTimerHandle` (`self.TimerHp`))
    (return)))

(fn `ResetHP`
  (set `self.Health` (`self.MaxHealth`))
  (set `self.IsDead` false))

(fn `StartHPRegaining`
  (bind _returnvalue (`KismetSystemLibrary.K2_SetTimerDelegate` (`|CreateDelegate` :!event `RegainingHealt`) (`self.RegainingHPForSeconds`) true (`self.DelayBeforeGetHeal`)))
  (set `self.TimerHp` _returnvalue))

(fn `TakeDamage`
  (params (DamageInfo :type "/Game/Blueprints/DamageSystem/S_DamageInfo Structure"))
  (bind (_amountofdamage _damagetype _damageresponse) (break `/Game/Blueprints/DamageSystem/S_DamageInfo` DamageInfo))
  (`self.CanBeDamaged`
    (:`DoDamage`
      (`KismetSystemLibrary.K2_ClearAndInvalidateTimerHandle` (`self.TimerHp`))
      (bind _output_get (set `self.Health` (- (`self.Health`) _amountofdamage)))
      (if (<= _output_get 0.0)
        (set `self.IsDead` true)
        (`self.OnDeath`)
        (else
          (`self.OnDamageResponse` _damageresponse _damagetype _output_get)
          (`self.StartHPRegaining`)
          (return))))
    (:`NoDamage`
      (return))))