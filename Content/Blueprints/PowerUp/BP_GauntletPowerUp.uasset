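; BP_GauntletPowerUp is a one-time power-up that raises the gauntlet's maximum light count.
; When its sphere is overlapped by a BP_Gauntlet, it adds its increment to that gauntlet's max, refreshes the HUD's slot and light displays, and calls the gauntlet to enable the light segment.
; It then clears its interactable flag to block repeat pickups, without destroying or hiding the actor.
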(event `self.Sphere.OnComponentBeginOverlap`
  (params (OverlappedComponent :type "PrimitiveComponent Object Reference") (OtherActor :type "Actor Object Reference") (OtherComp :type "PrimitiveComponent Object Reference") (OtherBodyIndex :type Integer) (bFromSweep :type Boolean) (SweepResult :type "HitResult Structure (by ref)"))
  (if (`self.IsInteractable`)
    (bind _asbp_gauntlett (cast `/Game/Blueprints/InteractionSystem/Gauntlet/BP_Gauntlet` OtherActor))
    (bind _output_get (set `/Game/Blueprints/InteractionSystem/BP_StoringLightBase.CurrentMaxLight` (+ (`/Game/Blueprints/InteractionSystem/BP_StoringLightBase.CurrentMaxLight` _asbp_gauntlett) (`self.IncrementLightCount`)) _asbp_gauntlett))
    (bind _hud_widget (`/Game/Blueprints/UI/HUD/AC_HUDGauntlet.HUD WIdget` (`/Game/Blueprints/InteractionSystem/Gauntlet/BP_Gauntlet.AC_HUDGauntlet` _asbp_gauntlett)))
    (`/Game/Blueprints/UI/HUD/WBP_HUDGauntlet.UpdateCurrentSlots` _hud_widget _output_get)
    (`/Game/Blueprints/UI/HUD/WBP_HUDGauntlet.UpdateCurrentLights` _hud_widget (`KismetArrayLibrary.Array_Length` (`/Game/Blueprints/InteractionSystem/BP_StoringLightBase.CurrentLights` _asbp_gauntlett)))
    (`/Game/Blueprints/InteractionSystem/Gauntlet/BP_Gauntlet.EnableLightSegmento` _asbp_gauntlett _output_get)
    (set `self.IsInteractable` false)))

(fn `UserConstructionScript`)