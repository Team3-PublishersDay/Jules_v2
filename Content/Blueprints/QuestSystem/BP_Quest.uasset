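; BP_Quest is a composite quest actor that completes once every quest part in its SubQuestList is complete.
; On BeginPlay it attaches each sub-quest to itself and binds that sub-quest's completion event to CheckQuest.
; When all report completed, it tries to activate dialogue and use quest data, then marks itself completed and fires its own OnComplete.
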(event `self.ReceiveBeginPlay`
  (for _array_element (`self.SubQuestList`)
    (`self.K2_AttachToActor` _array_element self "None" "KeepRelative" "KeepRelative" "KeepRelative" true)
    (add `self.OnComplete` _array_element (delegate `CheckQuest`))))

(event `CheckQuest`
  (bind _iscompleted (`self.CheckQuestCompleted`))
  (if _iscompleted
    (`|ExecutionSequence`
      (:`then_0`
        (`self.TryActivateDialogue`)
        (`self.TryUseQuestData`))
      (:`then_1`
        (set `self.isCompleted` true)
        (`self.OnComplete`)))))

(fn `CheckQuestCompleted`
  (returns (isCompleted :type Boolean))
  (locals (Completed :type Boolean :default false))
  (for _array_element (`self.SubQuestList`)
    (if (== (`/Game/Blueprints/QuestSystem/BP_QuestBase.isCompleted` _array_element) true)
      (set `local.Completed` true)
      (else
        (set `local.Completed` false)
        (break))))
  (return (`local.Completed`)))

(fn `UserConstructionScript`)