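; BP_SubQuest is a quest-system actor that groups quest parts and completes once all of them are done.
; On BeginPlay it attaches each entry in SubQuestPartList to itself and binds their completion events to CheckSubQuest.
; When every part is completed, it tries to activate dialogue and use quest data, then marks itself completed and fires its own completion call.
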(event `self.ReceiveBeginPlay`
  (for _array_element (`self.SubQuestPartList`)
    (`self.K2_AttachToActor` _array_element self "None" "KeepRelative" "KeepRelative" "KeepRelative" true)
    (add `self.OnComplete` _array_element (delegate `CheckSubQuest`))))

(event `CheckSubQuest`
  (bind _iscompleted (`self.CheckSubQuestCompleted`))
  (if _iscompleted
    (`|ExecutionSequence`
      (:`then_0`
        (`self.TryActivateDialogue`)
        (`self.TryUseQuestData`))
      (:`then_1`
        (set `self.isCompleted` true)
        (`self.OnComplete`)))))

(fn `CheckSubQuestCompleted`
  (returns (isCompleted :type Boolean))
  (locals (completed :type Boolean :default false))
  (for _array_element (`self.SubQuestPartList`)
    (if (== (`/Game/Blueprints/QuestSystem/BP_QuestBase.isCompleted` _array_element) true)
      (set `local.completed` true)
      (else
        (set `local.completed` false)
        (break))))
  (return (`local.completed`)))

(fn `UserConstructionScript`)