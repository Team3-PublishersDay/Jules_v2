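; BP_QuestBase is a base quest Blueprint that tracks whether a quest is completed and persists that state.
; Through saver component events, it writes and reads the completion flag in the save game's Quest map, keyed by Id.
; BeginPlay also restores the flag and fires completion if set; a later load only updates it.
; Helper functions fire optional dialogue triggers and play the quest part's feedback sound at the player.
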(event `self.ReceiveBeginPlay`
  (bind _savegame (`/Game/Blueprints/Saves/BPC_Saver.SaveGame` (`self.BPC_Saver`))
    (:`then`
      (`self.UseQuestSave` _savegame)
      (if (`self.isCompleted`)
        (`self.OnComplete`)))
    (:`else`)))

(event `self.BPC_Saver.OnGameLoaded`
  (params (SaveData :type "/Game/Blueprints/Saves/BP_DefaultSaveGame Object Reference"))
  (`self.UseQuestSave` SaveData))

(event `self.BPC_Saver.OnRequestSave`
  (params (SaveGame :type "/Game/Blueprints/Saves/BP_DefaultSaveGame Object Reference"))
  (`self.Save` SaveGame))

(fn `Save`
  (params (SaveGame :type "/Game/Blueprints/Saves/BP_DefaultSaveGame Object Reference"))
  (`BlueprintMapLibrary.Map_Add` (`/Game/Blueprints/Saves/BP_DefaultSaveGame.Quest` SaveGame) (`self.Id`) (`self.isCompleted`)))

(fn `TryActivateDialogue`
  (bind _dialoguetrigger (`self.DialogueTrigger`))
  (bind _dialoguetriggerafter (`self.DialogueTriggerAfter`))
  (`/Engine/EditorBlueprintResources/StandardMacros.IsValid` _dialoguetrigger
    (:`Is Valid`
      (`/Game/Blueprints/DialogueSystem/Triggers/BP_DialogueTrigger.OnDialogueTrig` _dialoguetrigger))
    (:`Is Not Valid`
      _))
  (`/Engine/EditorBlueprintResources/StandardMacros.IsValid` _dialoguetriggerafter
    (:`Is Valid`
      (`/Game/Blueprints/DialogueSystem/Triggers/BP_DialogueTriggerAfterQuestFinished.OnDialogueTrig` _dialoguetriggerafter)
      (return))
    (:`Is Not Valid`
      (return))))

(fn `TryUseQuestData`
  (`/Engine/EditorBlueprintResources/StandardMacros.IsValid` (`self.QuestPartData`)
    (:`Is Valid`
      (bind _asbp_player (cast `/Game/Blueprints/Player/BP_Player` (`GameplayStatics.GetPlayerPawn` 0)))
      (`GameplayStatics.PlaySoundAtLocation` (`/Game/Blueprints/QuestSystem/DA_QuestData.AudioFeedBack` (`self.QuestPartData`)) (`SceneComponent.K2_GetComponentLocation` (`Character.Mesh` _asbp_player)) (struct) 1.0 1.0 0.0 null null null null))))

(fn `UseQuestSave`
  (params (SaveGame :type "/Game/Blueprints/Saves/BP_DefaultSaveGame Object Reference"))
  (set `self.isCompleted` (`BlueprintMapLibrary.Map_Find` (`/Game/Blueprints/Saves/BP_DefaultSaveGame.Quest` SaveGame) (`self.Id`))))

(fn `UserConstructionScript`)