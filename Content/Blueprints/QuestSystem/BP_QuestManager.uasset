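; BP_QuestManager is an actor that tracks a list of quests and signals when all of them are completed.
; On BeginPlay it attaches each quest actor in QuestList to itself and binds to that quest's OnComplete event.
; Each completion rechecks the whole list, stopping at the first unfinished quest, and fires OnCompletedAllQuest if every quest is done.
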(event `self.ReceiveBeginPlay`
  (for _array_element (`self.QuestList`)
    (`self.K2_AttachToActor` _array_element self "None" "KeepRelative" "KeepRelative" "KeepRelative" true)
    (add `/Game/Blueprints/QuestSystem/BP_QuestBase.OnComplete` _array_element (delegate `CheckAllQuest`))))

(event `CheckAllQuest`
  (bind _areallcompleted (`self.CheckAllQuestCompleted`))
  (if _areallcompleted
    (`self.OnCompletedAllQuest`)))

(fn `CheckAllQuestCompleted`
  (returns (areAllCompleted :type Boolean))
  (locals (areCompleted :type Boolean :default false))
  (for _array_element (`self.QuestList`)
    (if (== (`/Game/Blueprints/QuestSystem/BP_QuestBase.isCompleted` _array_element) true)
      (set `local.areCompleted` true)
      (else
        (set `local.areCompleted` false)
        (break))))
  (return (`local.areCompleted`)))

(fn `UserConstructionScript`)