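; Player camera component that drives head bob and health-based post-process effects on BP_Player.
; Each tick it picks idle, walk or sprint camera shakes, with crouched variants, from movement speed, crouch state and CanJump, and starts them on player controller 0.
; SetHealthVFX raises post-process blend weight as health drops relative to the damage system's MaxHealth, while SetPostProcess sets that weight directly.
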(event `self.ReceiveBeginPlay`
  ;[1 1 1] Get player
  (bind _asbp_player (cast `/Game/Blueprints/Player/BP_Player` (`self.GetOwner`)))
  (set `self.As BP Player` _asbp_player))

(event `self.ReceiveTick`
  (params (DeltaSeconds :type "Float (single-precision)"))
  ;[1 0.807 0] Update Headbob
  (`self.SetHeadBob`))

(fn `GetVelocityLenght`
  (returns (ReturnValue :type "Float (double-precision)"))
  (return (`KismetMathLibrary.VSize` (`CharacterMovementComponent.GetLastUpdateVelocity` (`Character.CharacterMovement` (`self.As BP Player`))))))

(fn `SetHeadBob`
  (if (`Character.bIsCrouched` (`self.As BP Player`))
    (`self.SetHeadBobWhileCrouched`)
    (else
      (`self.SetHeadBobWhileWalk`))))

(fn `SetHeadBobWhileCrouched`
  (bind _returnvalue (`GameplayStatics.GetPlayerController` 0))
  (if (and (> (`self.GetVelocityLenght`) 0.0) (`Character.CanJump` (`self.As BP Player`)))
    (if (<= (`self.GetVelocityLenght`) (`/Game/Blueprints/Player/BP_Player.Max Walk Speed Crouched` (`self.As BP Player`)))
      (`PlayerController.ClientStartCameraShake` :`self` _returnvalue :`Shake` "/Game/Blueprints/Player/Camera/BP_CameraWalkCrouch.BP_CameraWalkCrouch_C")
      (else
        (`PlayerController.ClientStartCameraShake` :`self` _returnvalue :`Shake` "/Game/Blueprints/Player/Camera/BP_CameraSprintCrouch.BP_CameraSprintCrouch_C")))
    (else
      (`PlayerController.ClientStartCameraShake` :`self` _returnvalue :`Shake` "/Game/Blueprints/Player/Camera/BP_CameraIdleCrouch.BP_CameraIdleCrouch_C"))))

(fn `SetHeadBobWhileWalk`
  (bind _returnvalue (`GameplayStatics.GetPlayerController` 0))
  (if (and (> (`self.GetVelocityLenght`) 0.0) (`Character.CanJump` (`self.As BP Player`)))
    (if (<= (`self.GetVelocityLenght`) (`/Game/Blueprints/Player/BP_Player.Max Walk Speed` (`self.As BP Player`)))
      (`PlayerController.ClientStartCameraShake` :`self` _returnvalue :`Shake` "/Game/Blueprints/Player/Camera/BP_CameraWalk.BP_CameraWalk_C")
      (else
        (`PlayerController.ClientStartCameraShake` :`self` _returnvalue :`Shake` "/Game/Blueprints/Player/Camera/BP_CameraSprint.BP_CameraSprint_C")))
    (else
      (`PlayerController.ClientStartCameraShake` :`self` _returnvalue :`Shake` "/Game/Blueprints/Player/Camera/BP_CameraIdle.BP_CameraIdle_C"))))

(fn `SetHealthVFX`
  (params (Healt :type "Float (double-precision)"))
  (set `PostProcessComponent.BlendWeight` (- 1.0 (/ Healt (`/Game/Blueprints/DamageSystem/BPC_DamageSystem.MaxHealth` (`/Game/Blueprints/Player/BP_Player.BPC_DamageSystem` (`self.As BP Player`))))) (`/Game/Blueprints/Player/BP_Player.PostProcess` (`self.As BP Player`))))

(fn `SetPostProcess`
  (params (`PostProcess Weight` :type "Float (double-precision)"))
  (set `PostProcessComponent.BlendWeight` `PostProcess Weight` (`/Game/Blueprints/Player/BP_Player.PostProcess` (`self.As BP Player`))))