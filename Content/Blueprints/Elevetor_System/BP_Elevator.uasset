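; Two-floor elevator actor with clickable floor buttons and two gates that open when linked quest gates complete.
; Button clicks drive timelines that lerp the actor to its start position or by the Floor1 offset, zeroing player walk speed during travel.
; While BP_Player overlaps the trigger, Tick centers the mouse and enables click events.
; OpenGate moves gates in one lerp step using duration as alpha; CheckActualFloor has no effect.
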(event `self.ReceiveBeginPlay`
  ;[1 1 1] Quest System Management
  (`|ExecutionSequence`
    (:`then_0`
      (`/Engine/EditorBlueprintResources/StandardMacros.IsValid` (`self.Linked Quest Gate 1`)
        (:`Is Valid`
          (add `/Game/Blueprints/QuestSystem/BP_QuestBase.OnComplete` (`self.Linked Quest Gate 1`) (delegate `OpenGate1`)))))
    (:`then_1`
      (`/Engine/EditorBlueprintResources/StandardMacros.IsValid` (`self.Linked Quest Gate 2`)
        (:`Is Valid`
          (add `/Game/Blueprints/QuestSystem/BP_QuestBase.OnComplete` (`self.Linked Quest Gate 2`) (delegate `OpenGate2`)))))
    (:`then_2`
      (set `self.Floor 0 Position` (`self.K2_GetActorLocation`)))))

(event `self.floor 0.OnClicked`
  (params (TouchedComponent :type "PrimitiveComponent Object Reference") (ButtonPressed :type "Key Structure"))
  (bind _player (`self.Player`))
  ;[1 1 1] Buttons Interaction
  (if (not (`self.isMoving`))
    (`|ExecutionSequence`
      (:`then_0`
        (set `self.isMoving` true))
      (:`then_1`
        (set `self.Max Walk Speed` (`/Game/Blueprints/Player/BP_Player.Max Walk Speed` _player))
        (set `/Game/Blueprints/Player/BP_Player.Max Walk Speed` 0.0 _player))
      (:`then_2`
        (`self.CheckActualFloor` (`self.Floor 0 Position`))
        (bind _output_get (set `self.StartPos` (`self.K2_GetActorLocation`)))
        (bind _output_get_2 (set `self.TargetPos` (`self.Floor 0 Position`)))
        (bind (_direction _value) (`Timeline|Movement` :!via `PlayFromStart`)
          (:`Update`
            (`self.K2_SetActorLocation` (`KismetMathLibrary.VLerp` _output_get _output_get_2 _value)))
          (:`Finished`
            (set `self.isMoving` false)
            (set `/Game/Blueprints/Player/BP_Player.Max Walk Speed` (`self.Max Walk Speed`) (`self.Player`))))))))

(event `OpenGate1`
  ;[1 1 1] Quest System Management
  (`self.OpenGate` (`self.gate zone 1`) (`self.Gate 1 Open Location`) (`self.Gate 1 Opening Duration`))
  (`KismetSystemLibrary.PrintString` "gate 1 opened"))

(event `OpenGate2`
  ;[1 1 1] Quest System Management
  (`self.OpenGate` (`self.gate zone 2`) (`self.Gate 2 Open Location`) (`self.Gate 2 Opening Duration`))
  (`KismetSystemLibrary.PrintString` "gate 2 opened"))

(event `self.floor 1.OnClicked`
  (params (TouchedComponent :type "PrimitiveComponent Object Reference") (ButtonPressed :type "Key Structure"))
  (bind _returnvalue (`self.K2_GetActorLocation`))
  (bind _player (`self.Player`))
  ;[1 1 1] Buttons Interaction
  (if (not (`self.isMoving`))
    (`|ExecutionSequence`
      (:`then_0`
        (set `self.isMoving` true))
      (:`then_1`
        (set `self.Max Walk Speed` (`/Game/Blueprints/Player/BP_Player.Max Walk Speed` _player))
        (set `/Game/Blueprints/Player/BP_Player.Max Walk Speed` 0.0 _player))
      (:`then_2`
        (`self.CheckActualFloor` (`self.Floor 1 Position`))
        (bind _output_get (set `self.StartPos` _returnvalue))
        (bind _output_get_2 (set `self.TargetPos` (+ _returnvalue (`self.Floor 1 Position`))))
        (bind (_direction _value) (`Timeline|Timeline` :!via `PlayFromStart`)
          (:`Update`
            (`self.K2_SetActorLocation` (`KismetMathLibrary.VLerp` _output_get _output_get_2 _value)))
          (:`Finished`
            (set `self.isMoving` false)
            (set `/Game/Blueprints/Player/BP_Player.Max Walk Speed` (`self.Max Walk Speed`) (`self.Player`))))))))

(event `self.PlayerTrigger.OnComponentBeginOverlap`
  (params (OverlappedComponent :type "PrimitiveComponent Object Reference") (OtherActor :type "Actor Object Reference") (OtherComp :type "PrimitiveComponent Object Reference") (OtherBodyIndex :type Integer) (bFromSweep :type Boolean) (SweepResult :type "HitResult Structure (by ref)"))
  (bind _asbp_player (cast `/Game/Blueprints/Player/BP_Player` OtherActor))
  (set `self.PlayerIsOn` true)
  (set `self.Player` _asbp_player))

(event `self.PlayerTrigger.OnComponentEndOverlap`
  (params (OverlappedComponent :type "PrimitiveComponent Object Reference") (OtherActor :type "Actor Object Reference") (OtherComp :type "PrimitiveComponent Object Reference") (OtherBodyIndex :type Integer))
  (cast `/Game/Blueprints/Player/BP_Player` OtherActor)
  (set `self.PlayerIsOn` false))

(event `self.ReceiveTick`
  (params (DeltaSeconds :type "Float (single-precision)"))
  (bind _returnvalue (`GameplayStatics.GetPlayerController` 0))
  (bind (_returnvalue_x _returnvalue_y) (`KismetMathLibrary.BreakVector2D` (`WidgetLayoutLibrary.GetViewportSize`)))
  ;[1 1 1] Buttons Interaction
  (if (`self.PlayerIsOn`)
    (`PlayerController.SetMouseLocation` _returnvalue (`KismetMathLibrary.FTrunc` (/ _returnvalue_x 2.0)) (`KismetMathLibrary.FTrunc` (/ _returnvalue_y 2.0)))
    (set `PlayerController.bEnableClickEvents` true _returnvalue)))

(fn `CheckActualFloor`
  (params (A :type "Vector Structure"))
  (if (not (== A (`self.K2_GetActorLocation`)))
    (return)))

(fn `OpenGate`
  (params (GateToOpen :type "StaticMeshComponent Object Reference") (`Gate Open Location` :type "Vector Structure") (`Gate Opening Duration` :type "Float (single-precision)"))
  (`SceneComponent.K2_SetRelativeLocation` GateToOpen (`KismetMathLibrary.VLerp` (`SceneComponent.RelativeLocation` GateToOpen) `Gate Open Location` `Gate Opening Duration`) false false))

(fn `UserConstructionScript`)