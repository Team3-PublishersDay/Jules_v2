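; BP_LevelManger is a level manager that streams the tutorial and two levels in and out as quests are completed.
; Each quest completion increments LevelIndex.
; When the player enters its box, that index selects a door to open, mostly after a delay, and which levels to load or unload.
; The saver component stores the index and BeginPlay reads it back, but OnGameLoaded resets it to zero, ignoring the saved value.
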(event `self.ReceiveBeginPlay`
  (for _array_element (`self.Quests`)
    (add `/Game/Blueprints/QuestSystem/BP_QuestBase.OnComplete` _array_element (`|CreateDelegate` :!event `OnComplete_Event`))
    (bind _savegame (`/Game/Blueprints/Saves/BPC_Saver.SaveGame` (`self.BPC_Saver`))
      (:`then`
        (set `self.LevelIndex` (`/Game/Blueprints/Saves/BP_DefaultSaveGame.CurrentLevelIndex` _savegame)))
      (:`else`))))

(event `OnComplete_Event`
  (`/Engine/EditorBlueprintResources/StandardMacros.IncrementInt` (`self.LevelIndex`)))

(event `self.Box.OnComponentBeginOverlap`
  (params (OverlappedComponent :type "PrimitiveComponent Object Reference") (OtherActor :type "Actor Object Reference") (OtherComp :type "PrimitiveComponent Object Reference") (OtherBodyIndex :type Integer) (bFromSweep :type Boolean) (SweepResult :type "HitResult Structure (by ref)"))
  (bind _levelindex (`self.LevelIndex`))
  (bind _output (`|GetArrayItem` (`self.Doors`) _levelindex))
  (cast `/Game/Blueprints/Player/BP_Player` OtherActor)
  (switch `int` _levelindex
    (:`0`
      (`KismetSystemLibrary.Delay` 35.0)
      (`/Game/Blueprints/LevelManager/BP_HUBDoor.Perform` _output)
      (`GameplayStatics.LoadStreamLevelBySoftObjectPtr` "/Game/Levels/Blockouts/FinalSubLevels/scn_Tutorial_Final.scn_Tutorial_Final" true))
    (:`1`
      (`KismetSystemLibrary.Delay` 18.0)
      (`/Game/Blueprints/LevelManager/BP_HUBDoor.Perform` _output)
      (`GameplayStatics.LoadStreamLevelBySoftObjectPtr` "/Game/Levels/Blockouts/FinalSubLevels/scn_Level2_Final.scn_Level2_Final" true)
      (`GameplayStatics.UnloadStreamLevelBySoftObjectPtr` "/Game/Levels/Blockouts/FinalSubLevels/scn_Tutorial_Final.scn_Tutorial_Final"))
    (:`2`
      (`KismetSystemLibrary.Delay` 10.0)
      (`/Game/Blueprints/LevelManager/BP_HUBDoor.Perform` _output)
      (`GameplayStatics.LoadStreamLevelBySoftObjectPtr` "/Game/Levels/Blockouts/FinalSubLevels/scn_Level1_Final.scn_Level1_Final" true)
      (`GameplayStatics.UnloadStreamLevelBySoftObjectPtr` "/Game/Levels/Blockouts/FinalSubLevels/scn_Level2_Final.scn_Level2_Final"))
    (:`3`
      (`/Game/Blueprints/LevelManager/BP_HUBDoor.Perform` _output)
      (`GameplayStatics.UnloadStreamLevelBySoftObjectPtr` "/Game/Levels/Blockouts/FinalSubLevels/scn_Level1_Final.scn_Level1_Final"))))

(event `self.BPC_Saver.OnRequestSave`
  (params (SaveGame :type "/Game/Blueprints/Saves/BP_DefaultSaveGame Object Reference"))
  (set `/Game/Blueprints/Saves/BP_DefaultSaveGame.CurrentLevelIndex` (`self.LevelIndex`) SaveGame))

(event `self.BPC_Saver.OnGameLoaded`
  (params (SaveData :type "/Game/Blueprints/Saves/BP_DefaultSaveGame Object Reference"))
  (set `self.LevelIndex` 0))

(fn `UserConstructionScript`)