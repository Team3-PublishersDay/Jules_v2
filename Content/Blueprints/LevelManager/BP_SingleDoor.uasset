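; BP_SingleDoor is a level door that swings a single mesh open around its yaw axis, starting at the closed angle with tick disabled.
; Perform records the current yaw, derives a duration from angle distance and RotateVelocity, then enables Tick, which lerps toward the open angle and snaps at the end.
; The timer increment is also scaled by RotateVelocity.
; EndPerform prepares closing values, but Tick contains no closing lerp.
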(event `self.ReceiveBeginPlay`
  (`self.SetActorTickEnabled` self false)
  (`self.Set Rotation` (`self.ClosedDoorZAngle`) (`self.StaticMesh1`)))

(event `self.ReceiveTick`
  (params (DeltaSeconds :type "Float (single-precision)"))
  (bind _staticmesh1 (`self.StaticMesh1`))
  (if (`self.CanPerform`)
    (`self.Lerp` (`self.StartLerpAngle`) (`self.OpenDoorZAngle`) _staticmesh1 _staticmesh1)
    (if (>= (`self.Timer`) (`self.LerpDuration`))
      (`self.Set Rotation` (`self.OpenDoorZAngle`) (`self.StaticMesh1`)))))

(fn `EndPerform`
  (set `self.CanPerform` false)
  (`self.SetLerpData`)
  (set `self.LerpDuration` (`self.GetLerpDuration` (`self.ClosedDoorZAngle`))))

(fn `GetLerpDuration`
  (params (`End Lerp Angle` :type "Float (double-precision)"))
  (returns (ReturnValue :type "Float (double-precision)"))
  (return (/ (`KismetMathLibrary.Abs` (- (`self.StartLerpAngle`) `End Lerp Angle`)) (`self.RotateVelocity`))))

(fn `IncrementTimer`
  (returns (NewTimer :type "Float (double-precision)"))
  (return (+ (* (`GameplayStatics.GetWorldDeltaSeconds`) (`self.RotateVelocity`)) (`self.Timer`))))

(fn `Lerp`
  (params (A :type "Float (double-precision)") (B :type "Float (double-precision)") (Target :type "SceneComponent Object Reference") (Target1 :type "SceneComponent Object Reference"))
  (bind (_relativerotation_roll _relativerotation_pitch) (`KismetMathLibrary.BreakRotator` (`SceneComponent.RelativeRotation` Target)))
  (bind _output_get (set `self.Timer` (`self.IncrementTimer`)))
  (`SceneComponent.K2_SetRelativeRotation` Target1 (`KismetMathLibrary.MakeRotator` _relativerotation_roll _relativerotation_pitch (`KismetMathLibrary.Lerp` A B (/ _output_get (`self.LerpDuration`)))) false false))

(fn `Perform`
  (`self.SetLerpData`)
  (set `self.LerpDuration` (`self.GetLerpDuration` (`self.OpenDoorZAngle`)))
  (set `self.CanPerform` true)
  (`self.SetActorTickEnabled` self true))

(fn `Set Rotation`
  (params (CurrentRotation :type "Float (double-precision)") (Target :type "SceneComponent Object Reference"))
  (`SceneComponent.K2_SetRelativeRotation` Target (`KismetMathLibrary.MakeRotator` 0.0 0.0 CurrentRotation) false false))

(fn `SetLerpData`
  (bind (_relativerotation_roll _relativerotation_pitch _relativerotation_yaw) (`KismetMathLibrary.BreakRotator` (`SceneComponent.RelativeRotation` (`self.StaticMesh1`))))
  (set `self.Timer` 0.0)
  (set `self.StartLerpAngle` _relativerotation_yaw))

(fn `UserConstructionScript`
  (`parent.UserConstructionScript`))