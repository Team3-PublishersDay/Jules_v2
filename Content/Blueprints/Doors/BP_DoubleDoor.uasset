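; BP_DoubleDoor is a double door that swings two leaves open and closed through OpenDoor and CloseDoor events.
; Each event drives two timelines through a sequence, playing them to open and reversing them to close.
; Their alphas lerp the relative yaw of Door and Door1 from opposite orientations to a shared angle.
; The timeline updates write conflicting values to ClosedDoor, false from one and true from the other, regardless of direction.
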(event `OpenDoor`
  (`|ExecutionSequence`
    (:`then_0`
      (bind (_direction _door_alpha) (`Timeline|Open/Close` :!label _label)
        (:`Update`
          (`SceneComponent.K2_SetRelativeRotation` (`self.Door`) (`KismetMathLibrary.RLerp` (struct) (struct :`Yaw` -90.0) _door_alpha) false false)
          (set `self.ClosedDoor` false))))
    (:`then_1`
      (bind (_direction_2 _door_alpha_2) (`Timeline|Timeline` :!label _label_2)
        (:`Update`
          (`SceneComponent.K2_SetRelativeRotation` (`self.Door1`) (`KismetMathLibrary.RLerp` (struct :`Yaw` -180.0) (struct :`Yaw` -90.0) _door_alpha_2) false false)
          (set `self.ClosedDoor` true))))))

(event `CloseDoor`
  (`|ExecutionSequence`
    (:`then_0`
      (goto _label :!via `Reverse`))
    (:`then_1`
      (goto _label_2 :!via `Reverse`))))

(fn `UserConstructionScript`)