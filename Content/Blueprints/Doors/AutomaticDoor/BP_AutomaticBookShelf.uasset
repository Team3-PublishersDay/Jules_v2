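; Automatic bookshelf door that continuously swings its static mesh between closed and open yaw angles, with no trigger.
; BeginPlay snaps it closed and starts opening; Tick interpolates yaw by the current stance.
; At each end it snaps to the target and waits on a Delay before Perform or EndPerform reverses it.
; Those functions derive lerp duration from angle distance and RotateVelocity, but capture the start angle from Pitch rather than Yaw.
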(event `self.ReceiveBeginPlay`
  (`self.SetRotation` (`self.ClosedDoorZAngle`))
  (`self.Perform`))

(event `self.ReceiveTick`
  (params (DeltaSeconds :type "Float (single-precision)"))
  (if (`|EnumEquality` (`self.DoorStance`) "NewEnumerator0")
    (`self.Lerp` (`self.StartLerpAngle`) (`self.OpenDoorZAngle`))
    (if (>= (`self.Timer`) (`self.LerpDuration`))
      (`self.SetRotation` (`self.OpenDoorZAngle`))
      (`KismetSystemLibrary.Delay` (`self.DelayAfterNextPerform`))
      (`self.EndPerform`))
    (else
      (`self.Lerp` (`self.StartLerpAngle`) (`self.ClosedDoorZAngle`))
      (if (>= (`self.Timer`) (`self.LerpDuration`))
        (`self.SetRotation` (`self.ClosedDoorZAngle`))
        (`KismetSystemLibrary.Delay` (`self.DelayAfterNextPerform`))
        (`self.Perform`)))))

(fn `EndPerform`
  (`self.SetLerpData`)
  (set `self.LerpDuration` (`self.GetLerpDuration` (`self.ClosedDoorZAngle`)))
  (set `self.DoorStance` "NewEnumerator1"))

(fn `GetLerpDuration`
  (params (EndLerpDuration :type "Float (double-precision)"))
  (returns (ReturnValue :type "Float (double-precision)"))
  (return (/ (`KismetMathLibrary.Abs` (- (`self.StartLerpAngle`) EndLerpDuration)) (`self.RotateVelocity`))))

(fn `IncrementTimer`
  (returns (NewTimer :type "Float (double-precision)"))
  (return (+ (* (`GameplayStatics.GetWorldDeltaSeconds`) (`self.RotateVelocity`)) (`self.Timer`))))

(fn `Lerp`
  (params (a :type "Float (double-precision)") (b :type "Float (double-precision)"))
  (bind (_relativerotation_roll _relativerotation_pitch) (`KismetMathLibrary.BreakRotator` (`SceneComponent.RelativeRotation` (`self.StaticMesh`))))
  (bind _output_get (set `self.Timer` (`self.IncrementTimer`)))
  (`SceneComponent.K2_SetRelativeRotation` (`self.StaticMesh`) (`KismetMathLibrary.MakeRotator` _relativerotation_roll _relativerotation_pitch (`KismetMathLibrary.Lerp` a b (/ _output_get (`self.LerpDuration`)))) false false))

(fn `Perform`
  (`self.SetLerpData`)
  (set `self.LerpDuration` (`self.GetLerpDuration` (`self.OpenDoorZAngle`)))
  (set `self.DoorStance` "NewEnumerator0"))

(fn `SetLerpData`
  (bind (_relativerotation_roll _relativerotation_pitch) (`KismetMathLibrary.BreakRotator` (`SceneComponent.RelativeRotation` (`self.StaticMesh`))))
  (set `self.Timer` 0.0)
  (set `self.StartLerpAngle` _relativerotation_pitch))

(fn `SetRotation`
  (params (`New Rotation Z (Yaw)` :type "Float (single-precision)"))
  (`SceneComponent.K2_SetRelativeRotation` (`self.StaticMesh`) (`KismetMathLibrary.MakeRotator` 0.0 0.0 `New Rotation Z (Yaw)`) false false))

(fn `UserConstructionScript`)