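; Interactable door actor that alternates between opening and closing on each Interact event.
; A FlipFlop selects OpenDoor or CloseDoor, whose logic is not defined here, and a DoOnce with a short delayed reset throttles the sound.
; A box collision enables input and shows two text prompts while the player character overlaps it, then reverses both on exit.
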(event `self.Interact`
  (`/Engine/EditorBlueprintResources/StandardMacros.FlipFlop`
    (:`A`
      (`self.OpenDoor`))
    (:`B`
      (`self.CloseDoor`)))
  (`/Engine/EditorBlueprintResources/StandardMacros.DoOnce` false :!label _label
    (:`Completed`
      (`GameplayStatics.PlaySoundAtLocation` null (0.0 0.0 0.0) (struct) 1.0 1.0 0.0 null null null null)
      (`KismetSystemLibrary.Delay` 0.2)
      (`TypedElementListLibrary.Reset` (struct))
      (goto _label :!via `Reset`))))

(event `self.BoxCollision.OnComponentBeginOverlap`
  (params (OverlappedComponent :type "PrimitiveComponent Object Reference") (OtherActor :type "Actor Object Reference") (OtherComp :type "PrimitiveComponent Object Reference") (OtherBodyIndex :type Integer) (bFromSweep :type Boolean) (SweepResult :type "HitResult Structure (by ref)"))
  (if (== OtherActor (`GameplayStatics.GetPlayerCharacter` 0))
    (`self.EnableInput` (`GameplayStatics.GetPlayerController` 0))
    (`SceneComponent.SetHiddenInGame` (`self.TextRender1`) false false)
    (`SceneComponent.SetHiddenInGame` (`self.TextRender`) false false)))

(event `self.BoxCollision.OnComponentEndOverlap`
  (params (OverlappedComponent :type "PrimitiveComponent Object Reference") (OtherActor :type "Actor Object Reference") (OtherComp :type "PrimitiveComponent Object Reference") (OtherBodyIndex :type Integer))
  (if (== OtherActor (`GameplayStatics.GetPlayerCharacter` 0))
    (`self.DisableInput` (`GameplayStatics.GetPlayerController` 0))
    (`SceneComponent.SetHiddenInGame` (`self.TextRender`) true false)
    (`SceneComponent.SetHiddenInGame` (`self.TextRender1`) true false)))

(fn `UserConstructionScript`
  (`parent.UserConstructionScript`))