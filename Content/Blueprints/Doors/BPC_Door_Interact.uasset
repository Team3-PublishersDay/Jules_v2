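; Interactable door Blueprint that the player opens and closes with the E key while standing nearby.
; Box collision overlap with the player character enables or disables the actor's input and shows or hides two text render prompts.
; A FlipFlop alternates each E press between OpenDoor and CloseDoor, which are called here but defined outside these graphs.
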(event `Key|E`
  (params (Key :type "Key Structure"))
  (:`Pressed`
    (`/Engine/EditorBlueprintResources/StandardMacros.FlipFlop`
      (:`A`
        (`self.OpenDoor`))
      (:`B`
        (`self.CloseDoor`)))))

(event `self.BoxCollision.OnComponentBeginOverlap`
  (params (OverlappedComponent :type "PrimitiveComponent Object Reference") (OtherActor :type "Actor Object Reference") (OtherComp :type "PrimitiveComponent Object Reference") (OtherBodyIndex :type Integer) (bFromSweep :type Boolean) (SweepResult :type "HitResult Structure (by ref)"))
  ;[1 1 1] Open & Close Door
  (if (== OtherActor (`GameplayStatics.GetPlayerCharacter` 0))
    (`self.EnableInput` (`GameplayStatics.GetPlayerController` 0))
    (`SceneComponent.SetHiddenInGame` (`self.TextRender1`) false false)
    (`SceneComponent.SetHiddenInGame` (`self.TextRender`) false false)))

(event `self.BoxCollision.OnComponentEndOverlap`
  (params (OverlappedComponent :type "PrimitiveComponent Object Reference") (OtherActor :type "Actor Object Reference") (OtherComp :type "PrimitiveComponent Object Reference") (OtherBodyIndex :type Integer))
  ;[1 1 1] Open & Close Door
  (if (== OtherActor (`GameplayStatics.GetPlayerCharacter` 0))
    (`self.DisableInput` (`GameplayStatics.GetPlayerController` 0))
    (`SceneComponent.SetHiddenInGame` (`self.TextRender`) true false)
    (`SceneComponent.SetHiddenInGame` (`self.TextRender1`) true false)))

(fn `UserConstructionScript`
  (`parent.UserConstructionScript`))