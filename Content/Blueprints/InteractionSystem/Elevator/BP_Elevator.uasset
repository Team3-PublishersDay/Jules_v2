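; Elevator actor that moves its mesh along a spline, running from BeginPlay or waiting for StartConnector, depending on Stance.
; While performing, Tick advances spline distance and reverses direction at either end after a delay.
; A player entering Box pauses travel, with its collision disabled during forward motion.
; A player entering Box1 has walking frozen while the elevator rides to the spline end, where walk speed is restored.
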(event `self.ReceiveBeginPlay`
  (set `self.CachedSpeed` (`self.Spline Speed`))
  (set `self.Direction` (`self.Spline Speed`))
  (if (`|EnumEquality` (`self.Stance`) "NewEnumerator0")
    (`self.SetActorTickEnabled` self true)
    (set `self.CanPerform` true)
    (else
      (`self.SetActorTickEnabled` self false)
      (set `self.CanPerform` false))))

(event `self.ReceiveTick`
  (params (DeltaSeconds :type "Float (single-precision)"))
  (bind _as_bp_player (`self.As BP Player`))
  (if (`self.CanPerform`)
    (if (> (`self.Spline Speed`) 0.0)
      (`PrimitiveComponent.SetCollisionEnabled` (`self.Box`) "NoCollision")
      (else
        (`PrimitiveComponent.SetCollisionEnabled` (`self.Box`) "QueryOnly")))
    (set `self.Distance ` (`self.GetDistance` (`GameplayStatics.GetWorldDeltaSeconds`)))
    (`self.PerformSpline`)
    (`self.SetSpeedDirection`)
    (else
      (set `self.Distance ` (`self.GetDistance` (`GameplayStatics.GetWorldDeltaSeconds`)))
      (`self.PerformSpline`)
      (set `self.Spline Speed` (`KismetMathLibrary.Abs` (`self.CachedSpeed`)))
      (if (>= (`self.Distance `) (`SplineComponent.GetSplineLength` (`self.Spline`)))
        (set `self.Spline Speed` 0.0)
        (set `/Game/Blueprints/Player/BP_Player.Max Walk Speed` (`/Game/Blueprints/Player/BP_Player.CachedSpeed` _as_bp_player) _as_bp_player)))))

(event `self.Box.OnComponentBeginOverlap`
  (params (OverlappedComponent :type "PrimitiveComponent Object Reference") (OtherActor :type "Actor Object Reference") (OtherComp :type "PrimitiveComponent Object Reference") (OtherBodyIndex :type Integer) (bFromSweep :type Boolean) (SweepResult :type "HitResult Structure (by ref)"))
  (cast `/Game/Blueprints/Player/BP_Player` OtherActor)
  (if (`self.CanPerform`)
    (set `self.Direction` (`self.Spline Speed`))
    (set `self.Spline Speed` 0.0)))

(event `self.Box.OnComponentEndOverlap`
  (params (OverlappedComponent :type "PrimitiveComponent Object Reference") (OtherActor :type "Actor Object Reference") (OtherComp :type "PrimitiveComponent Object Reference") (OtherBodyIndex :type Integer))
  (cast `/Game/Blueprints/Player/BP_Player` OtherActor)
  (if (`self.CanPerform`)
    (set `self.Spline Speed` (`self.Direction`))))

(event `self.Box1.OnComponentBeginOverlap`
  (params (OverlappedComponent :type "PrimitiveComponent Object Reference") (OtherActor :type "Actor Object Reference") (OtherComp :type "PrimitiveComponent Object Reference") (OtherBodyIndex :type Integer) (bFromSweep :type Boolean) (SweepResult :type "HitResult Structure (by ref)"))
  (bind _asbp_player (cast `/Game/Blueprints/Player/BP_Player` OtherActor))
  (if (`self.CanPerform`)
    (bind _output_get (set `self.As BP Player` _asbp_player))
    (set `/Game/Blueprints/Player/BP_Player.Max Walk Speed` 0.0 _output_get)
    (set `self.CanPerform` false)))

(event `/Game/Blueprints/InteractionSystem/LightInteract/Interface/BPI_Generator.StartConnector`
  (`self.Perform`))

(event `/Game/Blueprints/InteractionSystem/LightInteract/Interface/BPI_Generator.EndConnector`
  (`self.EndPerform`))

(fn `EndPerform`
  (set `self.CanPerform` false)
  (set `self.Spline Speed` 0.0))

(fn `GetDistance`
  (params (`Time ` :type "Float (double-precision)"))
  (returns (`Direction ` :type "Float (double-precision)"))
  (return (+ (* `Time ` (`self.Spline Speed`)) (`self.Distance `))))

(fn `Perform`
  (set `self.CanPerform` true)
  (set `self.Spline Speed` (`KismetMathLibrary.Abs` (`self.CachedSpeed`)))
  (`self.SetActorTickEnabled` self true))

(fn `PerformSpline`
  (`SceneComponent.K2_SetWorldTransform` (`self.StaticMesh`) (`KismetMathLibrary.MakeTransform` (.location (`SplineComponent.GetTransformAtDistanceAlongSpline` (`self.Spline`) (`self.Distance `) "World" false)) (`KismetMathLibrary.MakeRotator` 0.0) (`SceneComponent.RelativeScale3D` (`self.StaticMesh`))) false false))

(fn `UserConstructionScript`)