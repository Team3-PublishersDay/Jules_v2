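; BP_LeversInteract is a lever object in the interaction system that rotates when interacted with.
; It inherits its interaction flow from a parent Blueprint, passing BeginPlay, TryInteract and Interact through to it.
; On Interact, a timeline plays from the start and its LeverRotation track lerps StaticMesh1's relative rotation from zero toward a 90-degree turn.
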(event `self.ReceiveBeginPlay`
  (`parent.ReceiveBeginPlay`))

(event `/Game/Blueprints/InteractionSystem/BaseInteract/Interface/BPI_Interactable.TryInteract`
  (`parent.TryInteract`))

(event `/Game/Blueprints/InteractionSystem/BaseInteract/Interface/BPI_Interactable.Interact`
  (`parent.Interact`)
  (bind (_direction _leverrotation) (`Timeline|Timeline` :!via `PlayFromStart`)
    (:`Update`
      (`SceneComponent.K2_SetRelativeRotation` (`self.StaticMesh1`) (`KismetMathLibrary.RLerp` (struct) (struct :`Roll` 90.0) _leverrotation) false false))))

(fn `UserConstructionScript`
  (`parent.UserConstructionScript`))