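; BP_PapperInteract is an interactable object, likely a paper, that the player picks up to inspect and puts back when done.
; Interacting moves input from the player to this actor with the inspection mapping context, disables mesh collision and snaps the mesh to the player's Scene component.
; IA_Move rotates the mesh, marked as needing a fix.
; IA_Interact stops inspection, restoring input, collision and the StartPosition transform.
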(event `self.ReceiveBeginPlay`
  (`parent.ReceiveBeginPlay`))

(event `/Game/Blueprints/InteractionSystem/BaseInteract/Interface/BPI_Interactable.TryInteract`
  (`parent.TryInteract`))

(event `/Game/Blueprints/InteractionSystem/BaseInteract/Interface/BPI_Interactable.Interact`
  (`parent.Interact`)
  (`self.SwapPlayerInput`)
  (`PrimitiveComponent.SetCollisionEnabled` (`self.StaticMesh`) "NoCollision")
  (`self.SetNewPosition`))

(event `/Game/Blueprints/InteractionSystem/BaseInteract/Interface/BPI_Interactable.StopInteract`
  (`parent.StopInteract`)
  (`self.BackToInitialInput`)
  (`SceneComponent.K2_SetRelativeTransform` (`self.StaticMesh`) (`self.StartPosition`) false false)
  (`PrimitiveComponent.SetCollisionEnabled` (`self.StaticMesh`) "QueryAndPhysics"))

(event `EnhancedInput|/Game/Blueprints/Player/Input/IA_Interact`
  (params (ActionValue :type Boolean) (ElapsedSeconds :type "Float (double-precision)") (TriggeredSeconds :type "Float (double-precision)") (InputAction :type "InputAction Object Reference" :default "/Game/Blueprints/Player/Input/IA_Interact.IA_Interact"))
  (:`Triggered`
    (`/Game/Blueprints/InteractionSystem/BaseInteract/Interface/BPI_Interactable.StopInteract`)))

(event `EnhancedInput|/Game/Blueprints/Player/Input/IA_Move`
  (params (ActionValue :type "Vector2D Structure") (ElapsedSeconds :type "Float (double-precision)") (TriggeredSeconds :type "Float (double-precision)") (InputAction :type "InputAction Object Reference" :default "/Game/Blueprints/Player/Input/IA_Move.IA_Move"))
  ;[1 1 1] DA SISTEMARE
  (:`Triggered`
    (`SceneComponent.K2_AddRelativeRotation` (`self.StaticMesh`) (`KismetMathLibrary.MakeRotator` 0.0 ActionValue_Y ActionValue_X) false false)))

(fn `BackToInitialInput`
  (`self.DisableInput` (`GameplayStatics.GetPlayerController` 0))
  (`/Game/Blueprints/BP_GameMode.SwapContext` (cast `/Game/Blueprints/BP_GameMode` (`GameplayStatics.GetGameMode`) :!pure true) "/Game/Blueprints/Player/Input/IMC_Player.IMC_Player")
  (`self.EnableInput` (`self.As BP Player`) null))

(fn `SetNewPosition`
  (bind (_startposition_location _startposition_rotation _startposition_scale) (`KismetMathLibrary.BreakTransform` (`self.StartPosition`)))
  (bind (_returnvalue_location _returnvalue_rotation) (`KismetMathLibrary.BreakTransform` (`SceneComponent.K2_GetComponentToWorld` (`/Game/Blueprints/Player/BP_Player.Scene` (`self.As BP Player`)))))
  (`SceneComponent.K2_SetWorldTransform` (`self.StaticMesh`) (`KismetMathLibrary.MakeTransform` _returnvalue_location _returnvalue_rotation _startposition_scale) false false))

(fn `SwapPlayerInput`
  (`self.DisableInput` (`self.As BP Player`) (`GameplayStatics.GetPlayerController` 0))
  (`/Game/Blueprints/BP_GameMode.SwapContext` (cast `/Game/Blueprints/BP_GameMode` (`GameplayStatics.GetGameMode`) :!pure true) "/Game/Blueprints/Player/Input/IMC_Inspection.IMC_Inspection")
  (`self.EnableInput` (`GameplayStatics.GetPlayerController` 0)))

(fn `UserConstructionScript`
  (`parent.UserConstructionScript`))