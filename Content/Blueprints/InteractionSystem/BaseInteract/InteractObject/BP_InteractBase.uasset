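; Base interactable actor that shows a prompt when the player enters its box and displays a message on screen when interacted with.
; A CanInteract check caps the number of interactions, gating both the overlap prompt and TryInteract.
; A successful attempt fires Interact, which creates or reuses the info widget, and completes a linked quest part once if flagged.
; StopInteract collapses the message and restores the prompt.
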(event `self.ReceiveBeginPlay`
  (`self.SetInteracionData`))

(event `/Game/Blueprints/InteractionSystem/BaseInteract/Interface/BPI_Interactable.TryInteract`
  (`self.CanInteract`
    (:`CanInteract`
      (`/Engine/EditorBlueprintResources/StandardMacros.IncrementInt` (`self.CurrentInteract`)
        (:`  `
          (`/Game/Blueprints/InteractionSystem/BaseInteract/Interface/BPI_Interactable.Interact`)
          (if (`self.IsPartOfQuest`)
            (`/Game/Blueprints/QuestSystem/BP_SubQuestPart.CompletePart` (`self.SubQuestPart`))
            (set `self.IsPartOfQuest` false)))))))

(event `/Game/Blueprints/InteractionSystem/BaseInteract/Interface/BPI_Interactable.Interact`
  (`self.ShowInteractionWidget`))

(event `/Game/Blueprints/InteractionSystem/BaseInteract/Interface/BPI_Interactable.StopInteract`
  (`SceneComponent.SetVisibility` (`self.Einteract`) true false)
  (`self.HideInteraction`))

(event `self.Box.OnComponentBeginOverlap`
  (params (OverlappedComponent :type "PrimitiveComponent Object Reference") (OtherActor :type "Actor Object Reference") (OtherComp :type "PrimitiveComponent Object Reference") (OtherBodyIndex :type Integer) (bFromSweep :type Boolean) (SweepResult :type "HitResult Structure (by ref)"))
  (cast `/Game/Blueprints/Player/BP_Player` OtherActor)
  (`self.CanInteract`
    (:`CanInteract`
      (`self.Interaction Feedback` true))))

(event `self.Box.OnComponentEndOverlap`
  (params (OverlappedComponent :type "PrimitiveComponent Object Reference") (OtherActor :type "Actor Object Reference") (OtherComp :type "PrimitiveComponent Object Reference") (OtherBodyIndex :type Integer))
  (cast `/Game/Blueprints/Player/BP_Player` OtherActor)
  (`self.Interaction Feedback` false))

(event `Interaction Feedback`
  (params (`Want See` :type Boolean))
  (`SceneComponent.SetVisibility` (`self.Einteract`) `Want See` false))

(event `ShowInteractionWidget`
  (bind _interactionwidget (`self.InteractionWidget`)
    (:`then`
      (`/Game/Blueprints/Player/HUD/Interact/W_InteractionInfo.SetTextEvent` _interactionwidget (`self.MessageToThePlayer`))
      (`Widget.SetVisibility` _interactionwidget "Visible"))
    (:`else`
      (bind _returnvalue (`|CreateWidget` "/Game/Blueprints/Player/HUD/Interact/W_InteractionInfo.W_InteractionInfo_C"))
      (bind _output_get (set `self.InteractionWidget` _returnvalue))
      (`/Game/Blueprints/Player/HUD/Interact/W_InteractionInfo.SetTextEvent` _output_get (`self.MessageToThePlayer`))
      (`UserWidget.AddToViewport` _output_get 0))))

(event `HideInteraction`
  (`Widget.SetVisibility` (`self.InteractionWidget`) "Collapsed"))

(fn `SetInteracionData`
  (bind _asbp_player (cast `/Game/Blueprints/Player/BP_Player` (`GameplayStatics.GetPlayerPawn` 0)))
  (set `self.As BP Player` _asbp_player)
  (set `self.StartPosition` (`SceneComponent.GetRelativeTransform` (`self.StaticMesh`))))

(fn `UserConstructionScript`)