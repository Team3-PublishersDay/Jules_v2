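; Actor component on BP_Player that lets the player interact with objects in view.
; On IA_Interact it line traces on the Visibility channel from the player camera along its forward vector, up to MaxDistanceInteraction.
; A hit actor implementing BPI_Interactable receives TryInteractMessage, after which BP_GameMode's CallOnOpenMenu is called.
; BeginPlay caches the owning BP_Player for camera access.
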(event `self.ReceiveBeginPlay`
  (bind _asbp_player (cast `/Game/Blueprints/Player/BP_Player` (`self.GetOwner`)))
  (set `self.As BP Player` _asbp_player))

(event `EnhancedInput|/Game/Blueprints/Player/Input/IA_Interact`
  (params (ActionValue :type Boolean) (ElapsedSeconds :type "Float (double-precision)") (TriggeredSeconds :type "Float (double-precision)") (InputAction :type "InputAction Object Reference" :default "/Game/Blueprints/Player/Input/IA_Interact.IA_Interact"))
  (bind (_start _end) (`self.GetRaycastPosition`))
  (:`Triggered`
    (bind _outhit (`KismetSystemLibrary.LineTraceSingle` _start _end "TraceTypeQuery1"))
    (bind (_bblockinghit _binitialoverlap _time _distance _location _impactpoint _normal _impactnormal _physmat _hitactor) (`GameplayStatics.BreakHitResult` _outhit))
    (if (`KismetSystemLibrary.DoesImplementInterface` _hitactor "/Game/Blueprints/InteractionSystem/BaseInteract/Interface/BPI_Interactable.BPI_Interactable_C")
      (message `/Game/Blueprints/InteractionSystem/BaseInteract/Interface/BPI_Interactable.TryInteract` _hitactor)
      (`/Game/Blueprints/BP_GameMode.OnOpenMenu` (cast `/Game/Blueprints/BP_GameMode` (`GameplayStatics.GetGameMode`) :!pure true)))))

(fn `GetRaycastPosition`
  (returns (Start :type "Vector Structure") (End :type "Vector Structure"))
  (bind _start (`self.GetStartRaycastPosition`))
  (return _start (+ _start (* (`KismetMathLibrary.GetForwardVector` (`SceneComponent.K2_GetComponentRotation` (`/Game/Blueprints/Player/BP_Player.Camera` (`self.As BP Player`)))) (`self.MaxDistanceInteraction`)))))

(fn `GetStartRaycastPosition`
  (returns (Start :type "Vector Structure"))
  (return (`SceneComponent.K2_GetComponentLocation` (`/Game/Blueprints/Player/BP_Player.Camera` (`self.As BP Player`)))))