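; BP_StartLevel is a trigger volume that clears light and interaction state when the player's BP_Gauntlett overlaps its Box.
; It fires while CanInteract is true, then disables itself once the cast succeeds.
; It destroys the gauntlet's CurrentLights and zeroes the HUD light count.
; It then calls EndPerform on each RestartInteract entry and destroys any lights those entries hold.
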(event `self.Box.OnComponentBeginOverlap`
  (params (OverlappedComponent :type "PrimitiveComponent Object Reference") (OtherActor :type "Actor Object Reference") (OtherComp :type "PrimitiveComponent Object Reference") (OtherBodyIndex :type Integer) (bFromSweep :type Boolean) (SweepResult :type "HitResult Structure (by ref)"))
  (if (`self.CanInteract`)
    (bind _asbp_gauntlett (cast `/Game/Blueprints/InteractionSystem/BP_Gauntlett` OtherActor))
    (set `self.CanInteract` false)
    (bind _currentlights (`/Game/Blueprints/InteractionSystem/BP_StoringLightBase.CurrentLights` _asbp_gauntlett))
    (if (> (`KismetArrayLibrary.Array_Length` _currentlights) 0)
      (for _array_element _currentlights
        (`self.K2_DestroyActor` _array_element))
      (`KismetArrayLibrary.Array_Clear` _currentlights)
      (`/Game/Blueprints/UI/HUD/WBP_HUDGauntlet.UpdateCurrentLights` (`/Game/Blueprints/UI/HUD/AC_HUDGauntlet.HUD WIdget` (`/Game/Blueprints/InteractionSystem/BP_Gauntlett.AC_HUDGauntlet` _asbp_gauntlett)) 0))
    (if (> (`KismetArrayLibrary.Array_Length` (`self.RestartInteract`)) 0)
      (for _array_element_2 (`self.RestartInteract`)
        (`/Game/Blueprints/InteractionSystem/BP_InteractLightBase.EndPerform` _array_element_2)
        (bind _currentlights_2 (`/Game/Blueprints/InteractionSystem/BP_StoringLightBase.CurrentLights` _array_element_2))
        (if (> (`KismetArrayLibrary.Array_Length` _currentlights_2) 0)
          (for _array_element_3 _currentlights_2
            (`self.K2_DestroyActor` _array_element_3))
          (`KismetArrayLibrary.Array_Clear` _currentlights_2))))))

(fn `UserConstructionScript`)