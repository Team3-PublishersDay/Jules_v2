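; Base interactable that stores light actors and trades them with the player's Gauntlet, with empty Perform and EndPerform hooks for children.
; Try actions check capacity, move the last light between arrays with animation, ownership change and sound, then broadcast the new count.
; On BeginPlay it attaches progressively scaled ring actors, is interactable only if RequiredLight is positive, and calls Perform if its light count exceeds that requirement.
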(event `self.ReceiveBeginPlay`
  (`parent.ReceiveBeginPlay`)
  (`self.SetLightPosition`)
  (`self.InitializeRingsPosition`)
  (if (> (`self.RequiredLight`) 0)
    (set `self.IsIteractable` true)
    (`self.Initial Ring Perform Animation`)
    (else
      (set `self.IsIteractable` false)))
  (if (> (`self.AmmountOfLight`) (`self.RequiredLight`))
    (`self.Perform`)))

(event `StartAction`
  (params (Gauntlet :type "/Game/Blueprints/InteractionSystem/BP_Gauntlett Object Reference"))
  ;[0 0 0] Action
  ;;[1 0.9292 0] Start Action
  (`self.Get Light` Gauntlet)
  (`self.SetLightPosition`)
  (`self.PlaySound` (`self.GetLightSound`)))

(event `Get Light`
  (params (Gauntlet :type "/Game/Blueprints/InteractionSystem/BP_Gauntlett Object Reference"))
  (bind _currentlights (`/Game/Blueprints/InteractionSystem/BP_StoringLightBase.CurrentLights` Gauntlet))
  (bind _returnvalue (`KismetArrayLibrary.Array_LastIndex` (`/Game/Blueprints/InteractionSystem/BP_StoringLightBase.CurrentLights` Gauntlet)))
  (bind _output (`|GetArrayItem` _currentlights _returnvalue))
  ;[0 0 0] Interface
  ;;[1 0 0] Get Light
  (`/Game/Blueprints/InteractionSystem/Light/BP_Lights.LightAnimation` _output Gauntlet (`self.K2_GetActorLocation` Gauntlet) (`self.K2_GetActorLocation` self))
  (`/Game/Blueprints/InteractionSystem/Light/BP_Lights.SetOwnerInteract` _output self)
  (`KismetArrayLibrary.Array_Add` (`self.CurrentLights`) _output)
  (`KismetArrayLibrary.Array_Remove` _currentlights _returnvalue))

(event `/Game/Blueprints/InteractionSystem/LightInteract/Interface/BPI_LightsInteract.TryStartAction`
  (params (Gauntlet :type "/Game/Blueprints/InteractionSystem/BP_Gauntlett Object Reference"))
  ;[0 0 0] Action
  ;;[1 0.9732 0] Try start action
  (`self.CanGetLight` (`self.CurrentMaxLight`)
    (:`CanGetLight`
      (`self.StartAction` Gauntlet)
      (`self.OnStartAction` (`KismetArrayLibrary.Array_Length` (`self.CurrentLights`))))))

(event `Give Light`
  (params (Gauntlet :type "/Game/Blueprints/InteractionSystem/BP_Gauntlett Object Reference"))
  (bind _currentlights (`self.CurrentLights`))
  (bind _output (`|GetArrayItem` _currentlights (`KismetArrayLibrary.Array_LastIndex` _currentlights)))
  ;[0 0 0] Interface
  ;;[1 0 0] Give Light
  (`/Game/Blueprints/InteractionSystem/Light/BP_Lights.SetOwnerInteract` _output Gauntlet)
  (`/Game/Blueprints/InteractionSystem/Light/BP_Lights.LightAnimation` _output Gauntlet (`self.K2_GetActorLocation` self) (`self.K2_GetActorLocation` Gauntlet))
  (`KismetArrayLibrary.Array_Add` (`/Game/Blueprints/InteractionSystem/BP_StoringLightBase.CurrentLights` Gauntlet) _output)
  (`KismetArrayLibrary.Array_RemoveItem` _currentlights _output))

(event `EndAction`
  (params (Gauntlet :type "/Game/Blueprints/InteractionSystem/BP_Gauntlett Object Reference"))
  ;[0 0 0] Action
  ;;[1 0 0.1804] End Action
  (`self.Give Light` Gauntlet)
  (`self.PlaySound` (`self.TakeLightSound`)))

(event `/Game/Blueprints/InteractionSystem/LightInteract/Interface/BPI_LightsInteract.TryEndAction`
  (params (Gauntlet :type "/Game/Blueprints/InteractionSystem/BP_Gauntlett Object Reference"))
  ;[0 0 0] Action
  ;;[1 0 0.1804] Try End action
  (`self.CanGiveLight` 0
    (:`CanGiveLight`
      (`self.EndAction` Gauntlet)
      (`self.OnEndAction` (`KismetArrayLibrary.Array_Length` (`self.CurrentLights`))))))

(fn `EndPerform`)

(fn `Initial Ring Perform Animation`
  (if (and (> (`KismetArrayLibrary.Array_Length` (`self.CurrentLights`)) 0) (> (`KismetArrayLibrary.Array_Length` (`self.Rings`)) 0))
    (for _index (range (`self.RequiredLight`))
      (`/Game/Blueprints/InteractionSystem/BP_RingAnimation.PerformAnimation` (`|GetArrayItem` (`self.Rings`) _index)))
    (return)))

(fn `InitializeRingsPosition`
  (if (> (`KismetArrayLibrary.Array_Length` (`self.Rings`)) 0)
    (for (_array_element _array_index) (`self.Rings`)
      (`self.SetOwner` _array_element self)
      (`self.K2_AttachToActor` _array_element self "None" "SnapToTarget" "KeepWorld" "KeepWorld" true)
      (`self.K2_SetActorRelativeLocation` _array_element (`SceneComponent.RelativeLocation` (`self.Sphere`)) false true)
      (`self.SetActorRelativeScale3D` _array_element (`KismetMathLibrary.Conv_DoubleToVector` (`self.InitialScale`)))
      (set `self.InitialScale` (+ (`self.InitialScale`) (`self.VarietyScaleDelta`)))
      (set `/Game/Blueprints/InteractionSystem/BP_RingAnimation.Index` _array_index _array_element)
      (`/Game/Blueprints/InteractionSystem/BP_RingAnimation.Initialize` _array_element self))
    (return)
    (else
      (return))))

(fn `IsInteractable`
  (returns (IsInteractable :type Boolean))
  (return (`self.IsIteractable`)))

(fn `Perform`)

(fn `PlaySound`
  (params (Sound :type "SoundBase Object Reference"))
  (`GameplayStatics.PlaySoundAtLocation` Sound (`self.K2_GetActorLocation` self) (struct) 1.0 1.0 0.0 null null null null))

(fn `SetLightPosition`
  (`parent.SetLightPosition`)
  ;[0.1656 0 1] Check for Lights
  (`self.CanGiveLight` 0
    (:`CanGiveLight`
      ;[1 0.8394 0] For each light
      (for _array_element (`self.CurrentLights`)
        ;[1 0 0.3185] Set the position
        (`self.K2_SetActorLocation` _array_element (`SceneComponent.K2_GetComponentLocation` (`self.Scene`)) false true)))))

(fn `UserConstructionScript`
  (`parent.UserConstructionScript`))