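; Interaction-system ring actor that spins while active, driven by a light count and its own Index.
; Initialize binds to the passed object's start and end action events.
; StartAction starts a looping timer when Index is the newest light, and EndAction clears it once Index falls outside the count.
; Each tick adds per-axis angular velocity times the timer interval to the actor's rotation, applied as relative rotation.
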(event `Initialize`
  (params (NewParam :type "/Game/Blueprints/InteractionSystem/BP_InteractLightBase Object Reference"))
  (add `/Game/Blueprints/InteractionSystem/BP_InteractLightBase.OnStartAction` NewParam (`|CreateDelegate` :!event `StartAction`))
  (add `/Game/Blueprints/InteractionSystem/BP_InteractLightBase.OnEndAction` NewParam (`|CreateDelegate` :!event `EndAction`)))

(event `PerformAnimation`
  (bind _returnvalue (`KismetSystemLibrary.K2_SetTimerDelegate` (`|CreateDelegate` :!event `RingAnimation`) (`self.RotationVelocityTimer`) true))
  (set `self.AnimationTimer` _returnvalue))

(event `EndAnimation`
  (set `self.IsPerforming` false)
  (`KismetSystemLibrary.K2_ClearAndInvalidateTimerHandle` (`self.AnimationTimer`)))

(event `RingAnimation`
  (set `self.IsPerforming` true)
  (`self.K2_SetActorRelativeRotation` (`self.CalculateRotation`)))

(event `StartAction`
  (params (`Light Amount` :type Integer))
  (if (== (`self.Index`) (- `Light Amount` 1))
    (if (not (`self.IsPerforming`))
      (`self.PerformAnimation`))))

(event `EndAction`
  (params (`Light Amount` :type Integer))
  (if (>= (`self.Index`) `Light Amount`)
    (if (`self.IsPerforming`)
      (`self.EndAnimation`))
    (else
      (set `self.IsPerforming` false))))

(fn `CalculateRotation`
  (returns (ReturnValue :type "Rotator Structure"))
  (bind (_returnvalue_roll _returnvalue_pitch _returnvalue_yaw) (`KismetMathLibrary.BreakRotator` (`self.K2_GetActorRotation`)))
  (bind (_returnvalue_roll_2 _returnvalue_pitch_2 _returnvalue_yaw_2) (`KismetMathLibrary.BreakRotator` (`KismetMathLibrary.MakeRotator` (* (`self.AngularVelocityX`) (`self.RotationVelocityTimer`)) (* (`self.AngularVelocityY`) (`self.RotationVelocityTimer`)) (* (`self.AngularVelocityZ`) (`self.RotationVelocityTimer`)))))
  (return (`KismetMathLibrary.MakeRotator` (+ _returnvalue_roll _returnvalue_roll_2) (+ _returnvalue_pitch _returnvalue_pitch_2) (+ _returnvalue_yaw _returnvalue_yaw_2))))

(fn `UserConstructionScript`)