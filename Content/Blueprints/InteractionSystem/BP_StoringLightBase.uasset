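; Base Blueprint for an interactable that stores lights, holding them in its CurrentLights array.
; On BeginPlay it binds to the game mode's OnRestartLevel event, then initializes each stored light with itself as owner.
; GetLightSlot returns a zero vector and RestartLevel, called from OnRestart, is empty, so both act as placeholders in this base.
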(event `self.ReceiveBeginPlay`
  (bind _asbp_game_mode (cast `/Game/Blueprints/BP_GameMode` (`GameplayStatics.GetGameMode`)))
  (add `/Game/Blueprints/BP_GameMode.OnRestartLevel` _asbp_game_mode (`|CreateDelegate` :!event `OnRestart`))
  (`self.InizializeStoringLight`))

(event `OnRestart`
  (`self.RestartLevel`))

(fn `AmmountOfLight`
  (returns (CurrentLight :type Integer))
  (return (`KismetArrayLibrary.Array_Length` (`self.CurrentLights`))))

(fn `GetLightSlot`
  (returns (NewPosition :type "Vector Structure"))
  (return (0.0 0.0 0.0)))

(fn `InizializeStoringLight`
  (`|ExecutionSequence`
    (:`then_0`
      (`self.GetLightSlot`))
    (:`then_1`
      (`self.SetLightInitialOwner`))))

(fn `RestartLevel`)

(fn `SetLightInitialOwner`
  ;[1 0 0.75] Check for the lights
  (if (> (`self.AmmountOfLight`) 0)
    (for _array_element (`self.CurrentLights`)
      ;[0.484 1 0] Inizialize Light
      (`/Game/Blueprints/InteractionSystem/Light/BP_Lights.Inizialize` _array_element self)
      (`/Game/Blueprints/InteractionSystem/Light/BP_Lights.SetOwnerInteract` _array_element self))))

(fn `UserConstructionScript`)