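; Gauntlet pickup that attaches to the player's arm on overlap and carries lights up to a slot capacity.
; While worn, a per-tick trace finds BPI_LightsInteract targets and toggles the HUD prompt; inputs take or give lights, updating the gauntlet HUD.
; A torch input toggles its spotlight while lights are held.
; Restart clears lights; loading a taken gauntlet moves it to the saved player transform.
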(event `self.ReceiveBeginPlay`
  (`self.SetActorTickEnabled` self false)
  (`self.InitializeSpotLightData`)
  (`self.InitializeLightsPositions`)
  (`self.InizializeLightSegmento`)
  (`self.EnableLightSegmento` (`self.CurrentMaxLight`))
  (bind _asbp_game_mode (cast `/Game/Blueprints/BP_GameMode` (`GameplayStatics.GetGameMode`)))
  (add `/Game/Blueprints/BP_GameMode.OnRestartLevel` _asbp_game_mode (`|CreateDelegate` :!event `Restart`))
  (bind _savegame (`/Game/Blueprints/Saves/BPC_Saver.SaveGame` (`self.BPC_Saver`))
    (:`then`
      (`self.UseGauntletSave` _savegame))
    (:`else`)))

(event `self.Box.OnComponentBeginOverlap`
  (params (OverlappedComponent :type "PrimitiveComponent Object Reference") (OtherActor :type "Actor Object Reference") (OtherComp :type "PrimitiveComponent Object Reference") (OtherBodyIndex :type Integer) (bFromSweep :type Boolean) (SweepResult :type "HitResult Structure (by ref)"))
  (bind _hud_widget (`/Game/Blueprints/UI/HUD/AC_HUDGauntlet.HUD WIdget` (`self.AC_HUDGauntlet`)))
  ;[1 0 0] Attach To player
  (bind _asbp_player (cast `/Game/Blueprints/Player/BP_Player` OtherActor))
  (bind _output_get (set `self.As BP Player` _asbp_player))
  (set `/Game/Blueprints/Player/BP_Player.Gauntlet` self _output_get)
  (`self.InitializeInput`)
  (`self.SetActorTickEnabled` self true)
  (`self.K2_AttachToComponent` (`/Game/Blueprints/Player/BP_Player.Arm` (`self.As BP Player`)) "Gauntlet" "SnapToTarget" "SnapToTarget" "KeepWorld")
  (`/Game/Blueprints/UI/HUD/AC_HUDGauntlet.InitializeHUDGauntlet` (`self.AC_HUDGauntlet`))
  (`/Game/Blueprints/UI/HUD/WBP_HUDGauntlet.UpdateCurrentSlots` _hud_widget (`self.CurrentMaxLight`))
  (`/Game/Blueprints/UI/HUD/WBP_HUDGauntlet.UpdateCurrentLights` _hud_widget (`KismetArrayLibrary.Array_Length` (`self.CurrentLights`)))
  (`PrimitiveComponent.SetCollisionEnabled` (`self.Box`) "NoCollision")
  (if (not (`self.IsAlreadyTaking`))
    (`GameplayStatics.PlaySoundAtLocation` (`self.TakeGauntletSound`) (`self.K2_GetActorLocation`) (struct) 1.0 1.0 0.0 null null null null)
    (set `self.IsAlreadyTaking` true)))

(event `self.ReceiveTick`
  (params (DeltaSeconds :type "Float (single-precision)"))
  (`self.Raycast`))

(event `EnhancedInput|/Game/Blueprints/Player/Input/IA_TakeLight`
  (params (ActionValue :type Boolean) (ElapsedSeconds :type "Float (double-precision)") (TriggeredSeconds :type "Float (double-precision)") (InputAction :type "InputAction Object Reference" :default "/Game/Blueprints/Player/Input/IA_TakeLight.IA_TakeLight"))
  ;[1 0.9237 0] TAKE LIGHT TO THE OBJECT
  (:`Triggered`
    (`self.CanInteractWith`
      (:`True`
        (if (< (`self.AmmountOfLight`) (`self.CurrentMaxLight`))
          (`/Game/Blueprints/InteractionSystem/LightInteract/Interface/BPI_LightsInteract.TryEndAction` (`self.HitActor`) self)
          (`/Game/Blueprints/UI/HUD/WBP_HUDGauntlet.UpdateCurrentLights` (`/Game/Blueprints/UI/HUD/AC_HUDGauntlet.HUD WIdget` (`self.AC_HUDGauntlet`)) (`KismetArrayLibrary.Array_Length` (`self.CurrentLights`))))))))

(event `EnhancedInput|/Game/Blueprints/Player/Input/IA_GiveLight`
  (params (ActionValue :type Boolean) (ElapsedSeconds :type "Float (double-precision)") (TriggeredSeconds :type "Float (double-precision)") (InputAction :type "InputAction Object Reference" :default "/Game/Blueprints/Player/Input/IA_GiveLight.IA_GiveLight"))
  ;[1 0 0.2253] GIVE LIGHT TO THE OBJECT
  (:`Triggered`
    (`self.CanInteractWith`
      (:`True`
        (if (> (`self.AmmountOfLight`) 0)
          (`/Game/Blueprints/InteractionSystem/LightInteract/Interface/BPI_LightsInteract.TryStartAction` (`self.HitActor`) self)
          (`/Game/Blueprints/UI/HUD/WBP_HUDGauntlet.UpdateCurrentLights` (`/Game/Blueprints/UI/HUD/AC_HUDGauntlet.HUD WIdget` (`self.AC_HUDGauntlet`)) (`KismetArrayLibrary.Array_Length` (`self.CurrentLights`)))
          (if (not (> (`self.AmmountOfLight`) 0))
            (`SceneComponent.SetVisibility` (`self.SpotLight`) false false)))))))

(event `Restart`
  ;[0 0.2739 1] OnDeath
  (`self.As BP Player`
    (:`then`
      (`/Game/Blueprints/UI/HUD/WBP_HUDGauntlet.UpdateCurrentLights` (`/Game/Blueprints/UI/HUD/AC_HUDGauntlet.HUD WIdget` (`self.AC_HUDGauntlet`)) 0)
      (`KismetArrayLibrary.Array_Clear` (`self.CurrentLights`)))
    (:`else`)))

(event `EnhancedInput|/Game/Blueprints/Player/Input/IA_Torch`
  (params (ActionValue :type Boolean) (ElapsedSeconds :type "Float (double-precision)") (TriggeredSeconds :type "Float (double-precision)") (InputAction :type "InputAction Object Reference" :default "/Game/Blueprints/Player/Input/IA_Torch.IA_Torch"))
  ;[0.5984 1 0.4792] Tourch
  (:`Triggered`
    (if (> (`self.AmmountOfLight`) 0)
      (`/Engine/EditorBlueprintResources/StandardMacros.FlipFlop`
        (:`A`
          (`SceneComponent.SetVisibility` (`self.SpotLight`) true false))
        (:`B`
          (`SceneComponent.SetVisibility` (`self.SpotLight`) false false))))))

(event `GiveLightSoundEvent`
  ;[1 0 0.5492] Sound
  (`GameplayStatics.PlaySound2D` (`self.GiveLightSound`) 1.0 1.0 0.0 null null))

(event `GetLightSoundEvent`
  ;[1 0 0.5492] Sound
  (`GameplayStatics.PlaySound2D` (`self.GetLightSound`) 1.0 1.0 0.0 null null))

(event `PlayLightMontage`
  (params (MontageToPlay :type "AnimMontage Object Reference"))
  (`|PlayMontage` (`/Game/Blueprints/Player/BP_Player.Arm` (`self.As BP Player`)) MontageToPlay
    (:`then`
      (set `self.CanInteract` false)
      (`self.StartLightAnimation`))
    (:`OnCompleted`
      (set `self.CanInteract` true)
      (`self.EndLightAnimation`))))

(event `self.BPC_Saver.OnRequestSave`
  (params (SaveGame :type "/Game/Blueprints/Saves/BP_DefaultSaveGame Object Reference"))
  (`self.GetGauntletSave` SaveGame))

(event `self.BPC_Saver.OnGameLoaded`
  (params (SaveData :type "/Game/Blueprints/Saves/BP_DefaultSaveGame Object Reference"))
  (`self.UseGauntletSave` SaveData))

(fn `EnableLightSegmento`
  (params (CurrentMaxLight :type Integer))
  (for (_array_element _array_index) (`self.LightsSegmento`)
    (if (< _array_index CurrentMaxLight)
      (`SceneComponent.SetVisibility` _array_element true false)
      (else
        (break)))))

(fn `EndLightAnimation`
  (`self.EnableInput` (`self.As BP Player`) (`GameplayStatics.GetPlayerController` 0))
  (set `self.CanInteract` true))

(fn `GetFirstOccupedLight`
  (returns (`Relative Location` :type "Vector Structure"))
  (locals (LightsPositionRef :type "Array of /Game/Blueprints/InteractionSystem/Gauntlet/SC_LightsSlot Object Reference"))
  (bind _lightspositionref (`local.LightsPositionRef`))
  (set `local.LightsPositionRef` (`self.LightsPositions`))
  (`KismetArrayLibrary.Array_Reverse` _lightspositionref)
  (for _array_element _lightspositionref
    (if (`/Game/Blueprints/InteractionSystem/Gauntlet/SC_LightsSlot.IsOccuped` _array_element)
      (`/Game/Blueprints/InteractionSystem/Gauntlet/SC_LightsSlot.Dissocupy` _array_element)
      (break)))
  (return (`SceneComponent.K2_GetComponentLocation` _array_element)))

(fn `GetGauntletSave`
  (params (SaveGame :type "/Game/Blueprints/Saves/BP_DefaultSaveGame Object Reference"))
  (set `/Game/Blueprints/Saves/BP_DefaultSaveGame.GauntletSave` (make `/Game/Blueprints/Saves/GauntletSave/S_GauntletSave` (`self.IsAlreadyTaking`)) SaveGame))

(fn `GetLightSlot`
  (returns (NewPosition :type "Vector Structure"))
  (for _array_element (`self.LightsPositions`)
    (if (not (`/Game/Blueprints/InteractionSystem/Gauntlet/SC_LightsSlot.IsOccuped` _array_element))
      (`/Game/Blueprints/InteractionSystem/Gauntlet/SC_LightsSlot.Occuped` _array_element)
      (break)))
  (return (`SceneComponent.K2_GetComponentLocation` _array_element)))

(fn `InitializeInput`
  (bind _returnvalue (`GameplayStatics.GetPlayerController` 0))
  (`EnhancedInputSubsystemInterface.AddMappingContext` (pcsubsystem `EnhancedInputLocalPlayerSubsystem` _returnvalue) "/Game/Blueprints/Player/Input/IMC_Interaction.IMC_Interaction" 0 (struct))
  (`self.EnableInput` _returnvalue))

(fn `InitializeLightsPositions`
  (for _array_element (`SceneComponent.GetChildrenComponents` (`self.StaticMesh`) false)
    (bind _assc_lights_slot (cast `/Game/Blueprints/InteractionSystem/Gauntlet/SC_LightsSlot` _array_element))
    (`KismetArrayLibrary.Array_Add` (`self.LightsPositions`) _assc_lights_slot))
  (return))

(fn `InitializeSpotLightData`
  (`LightComponent.SetIntensity` (`self.SpotLight`) (`self.LightIntensity`))
  (`LightComponent.SetLightColor` (`self.SpotLight`) (`KismetMathLibrary.Conv_ColorToLinearColor` (`self.LightColor`)) true)
  (`SpotLightComponent.SetOuterConeAngle` (`self.SpotLight`) (`self.OuterConeAngle`))
  (`LocalLightComponent.SetAttenuationRadius` (`self.SpotLight`) (`self.AttenuationRadius`))
  (`SceneComponent.SetVisibility` (`self.SpotLight`) false false))

(fn `InitialSetUpOwner`
  (params (NewOwner :type "/Game/Blueprints/Player/BP_Player Object Reference"))
  (`self.SetOwner` NewOwner)
  (`self.K2_AttachToActor` NewOwner "None" "KeepRelative" "KeepRelative" "KeepRelative")
  (`self.K2_SetActorRelativeLocation` (70.0 50.0 10.0))
  (`self.K2_SetActorRelativeRotation` (struct))
  (`PrimitiveComponent.SetCollisionEnabled` (`self.Box`) "NoCollision"))

(fn `InizializeLightSegmento`
  (set `self.LightsSegmento` (`SceneComponent.GetChildrenComponents` (`self.LightSegmento`) false))
  (for _array_element (`self.LightsSegmento`)
    (`SceneComponent.SetVisibility` _array_element false false))
  (return))

(fn `PIppo`
  (returns (NewPosition :type "Vector Structure"))
  (for _array_element (`self.LightsPositions`)
    (if (not (`/Game/Blueprints/InteractionSystem/Gauntlet/SC_LightsSlot.IsOccuped` _array_element))
      (`/Game/Blueprints/InteractionSystem/Gauntlet/SC_LightsSlot.Occuped` _array_element)
      (break)))
  (return (`SceneComponent.K2_GetComponentLocation` _array_element)))

(fn `Raycast`
  (bind _camera (`/Game/Blueprints/Player/BP_Player.Camera` (`self.As BP Player`)))
  (bind _returnvalue (`SceneComponent.K2_GetComponentLocation` _camera))
  (bind _outhit (`KismetSystemLibrary.LineTraceSingle` _returnvalue (+ _returnvalue (* (`KismetMathLibrary.GetForwardVector` (`SceneComponent.K2_GetComponentRotation` _camera)) (`self.InteractionDistance`))) "TraceTypeQuery1" false (`|MakeArray` (`self.As BP Player`) self :!type "Actor Object Reference")))
  (bind _asbpi_lights_interact (cast `/Game/Blueprints/InteractionSystem/LightInteract/Interface/BPI_LightsInteract` (`.HitActor` (`GameplayStatics.BreakHitResult` _outhit)))
    (:`then`
      (bind _output_get (set `self.HitActor` _asbpi_lights_interact))
      (bind _isinteractable (`/Game/Blueprints/InteractionSystem/LightInteract/Interface/BPI_LightsInteract.IsInteractable` _output_get))
      (if _isinteractable
        (set `self.IsHitting` true)
        (bind _asbp_hud (cast `/Game/Blueprints/Player/BP_HUD` (`PlayerController.GetHUD` (`GameplayStatics.GetPlayerController` 0))))
        (`/Game/Blueprints/Player/HUD/Interact/W_LightInteract.SetVisibile` (`/Game/Blueprints/Player/BP_HUD.Player Interact` _asbp_hud))))
    (:`CastFailed`
      (set `self.HitActor` null)
      (set `self.IsHitting` false)
      (bind _asbp_hud_2 (cast `/Game/Blueprints/Player/BP_HUD` (`PlayerController.GetHUD` (`GameplayStatics.GetPlayerController` 0))))
      (`/Game/Blueprints/Player/HUD/Interact/W_LightInteract.Hide` (`/Game/Blueprints/Player/BP_HUD.Player Interact` _asbp_hud_2)))))

(fn `RestartLevel`
  (`parent.RestartLevel`)
  (if (> (`self.AmmountOfLight`) 0)
    (`KismetArrayLibrary.Array_Clear` (`self.CurrentLights`))))

(fn `SetLightInitialOwner`
  (`parent.SetLightInitialOwner`))

(fn `SetPosition`
  (for (_array_element _array_index) (`self.CurrentLights`)
    (`self.K2_SetActorLocation` _array_element (`SceneComponent.K2_GetComponentLocation` (`|GetArrayItem` (`self.LightsPositions`) _array_index)) false true))
  (return))

(fn `StartLightAnimation`
  (`self.DisableInput` (`self.As BP Player`) (`GameplayStatics.GetPlayerController` 0))
  (set `self.CanInteract` false))

(fn `UseGauntletSave`
  (params (SaveGame :type "/Game/Blueprints/Saves/BP_DefaultSaveGame Object Reference"))
  (bind _gauntletsave_isalreadytaken (break `/Game/Blueprints/Saves/GauntletSave/S_GauntletSave` (`/Game/Blueprints/Saves/BP_DefaultSaveGame.GauntletSave` SaveGame)))
  (bind _playersave_transform (break `/Game/Blueprints/Saves/PlayerSave/S_PlayerSave` (`/Game/Blueprints/Saves/BP_DefaultSaveGame.PlayerSave` SaveGame)))
  (if (== _gauntletsave_isalreadytaken true)
    (set `self.IsAlreadyTaking` _gauntletsave_isalreadytaken)
    (`self.K2_SetActorTransform` _playersave_transform false true)))

(fn `UserConstructionScript`
  (`parent.UserConstructionScript`))