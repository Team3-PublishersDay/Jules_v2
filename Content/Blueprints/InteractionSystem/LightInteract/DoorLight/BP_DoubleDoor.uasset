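; Double door in the light interaction system that swings two mirrored leaves open when it has the required light.
; Gauntlet actions check the light amount to open or close it, while connector events drive it when non-interactable or short of light.
; Tick lerps yaw from the current angle, scaling duration by remaining angle, and switches off once fully closed.
; Level restart clears its lights and snaps it shut.
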(event `self.ReceiveBeginPlay`
  (`self.SetActorTickEnabled` self false)
  (`self.Set Rotation` (`self.ClosedDoorZAngle`))
  (`parent.ReceiveBeginPlay`))

(event `self.StartAction`
  (params (Gauntlet :type "/Game/Blueprints/InteractionSystem/BP_Gauntlett Object Reference"))
  (`parent.StartAction` Gauntlet)
  (`self.HasRequiredLight`
    (:`HasRequiredLight`
      (`GameplayStatics.PlaySoundAtLocation` (`self.DoorSound`) (`self.K2_GetActorLocation` self) (struct) 1.0 1.0 0.0 null null null null)
      (`self.Perform`)
      (goto _label :!via `Reset`))))

(event `self.EndAction`
  (params (Gauntlet :type "/Game/Blueprints/InteractionSystem/BP_Gauntlett Object Reference"))
  (`parent.EndAction` Gauntlet)
  (`self.HasRequiredLight`
    (:`Doesen'tHaveRequiredLight`
      (`self.EndPerform`)
      (`/Engine/EditorBlueprintResources/StandardMacros.DoOnce` false :!label _label
        (:`Completed`
          (`GameplayStatics.PlaySoundAtLocation` (`self.DoorSound`) (`self.K2_GetActorLocation` self) (struct) 1.0 1.0 0.0 null null null null))))))

(event `self.ReceiveTick`
  (params (DeltaSeconds :type "Float (single-precision)"))
  (if (`self.CanPerform`)
    (`self.Lerp` (`self.StartLerpAngle`) (`self.OpenDoorZAngle`))
    (if (>= (`self.Timer`) (`self.LerpDuration`))
      (`self.Set Rotation` (`self.OpenDoorZAngle`)))
    (else
      (`self.Lerp` (`self.StartLerpAngle`) (`self.ClosedDoorZAngle`))
      (if (>= (`self.Timer`) (`self.LerpDuration`))
        (`self.Set Rotation` (`self.ClosedDoorZAngle`))
        (`self.SetActorTickEnabled` self false)))))

(event `self.StartConnector`
  (if (`self.IsIteractable`)
    (`self.HasRequiredLight`
      (:`Doesen'tHaveRequiredLight`
        _)))
  (`self.Perform`))

(event `self.EndConnector`
  (if (`self.IsIteractable`)
    (`self.HasRequiredLight`
      (:`Doesen'tHaveRequiredLight`
        _)))
  (`self.EndPerform`))

(fn `CalculateEndRotation`
  (params (DeltaAngle :type "Float (double-precision)"))
  (set `self.EndLerpAngle` (+ (`self.StartLerpAngle`) DeltaAngle)))

(fn `EndPerform`
  (`parent.EndPerform`)
  (set `self.CanPerform` false)
  (`self.SetLerpData`)
  (set `self.LerpDuration` (`self.GetLerpDuration` (`self.ClosedDoorZAngle`))))

(fn `GetLerpDuration`
  (params (`End Lerp Angle` :type "Float (double-precision)"))
  (returns (ReturnValue :type "Float (double-precision)"))
  (return (/ (`KismetMathLibrary.Abs` (- (`self.StartLerpAngle`) `End Lerp Angle`)) (`self.RotateVelocity`))))

(fn `IncrementTimer`
  (returns (NewTimer :type "Float (double-precision)"))
  (return (+ (* (`GameplayStatics.GetWorldDeltaSeconds`) (`self.RotateVelocity`)) (`self.Timer`))))

(fn `Lerp`
  (params (A :type "Float (double-precision)") (B :type "Float (double-precision)"))
  (bind (_relativerotation_roll _relativerotation_pitch) (`KismetMathLibrary.BreakRotator` (`SceneComponent.RelativeRotation` (`self.StaticMesh`))))
  (bind _output_get (set `self.Timer` (`self.IncrementTimer`)))
  (bind _returnvalue (`KismetMathLibrary.Lerp` A B (/ _output_get (`self.LerpDuration`))))
  (`SceneComponent.K2_SetRelativeRotation` (`self.StaticMesh`) (`KismetMathLibrary.MakeRotator` _relativerotation_roll _relativerotation_pitch _returnvalue) false false)
  (`SceneComponent.K2_SetRelativeRotation` (`self.StaticMesh1`) (`KismetMathLibrary.MakeRotator` _relativerotation_roll _relativerotation_pitch (* _returnvalue -1.0)) false false))

(fn `Perform`
  (`parent.Perform`)
  (set `self.CanPerform` true)
  (`self.SetLerpData`)
  (set `self.LerpDuration` (`self.GetLerpDuration` (`self.OpenDoorZAngle`)))
  (`self.SetActorTickEnabled` self true))

(fn `RestartLevel`
  (`parent.RestartLevel`)
  (`KismetArrayLibrary.Array_Clear` (`self.CurrentLights`))
  (set `self.CanPerform` false)
  (`self.Set Rotation` (`self.ClosedDoorZAngle`)))

(fn `Set Rotation`
  (params (CurrentRotation :type "Float (double-precision)"))
  (`SceneComponent.K2_SetRelativeRotation` (`self.StaticMesh`) (`KismetMathLibrary.MakeRotator` 0.0 0.0 CurrentRotation) false false)
  (`SceneComponent.K2_SetRelativeRotation` (`self.StaticMesh1`) (`KismetMathLibrary.MakeRotator` 0.0 0.0 (* CurrentRotation -1.0)) false false))

(fn `SetLerpData`
  (bind (_relativerotation_roll _relativerotation_pitch _relativerotation_yaw) (`KismetMathLibrary.BreakRotator` (`SceneComponent.RelativeRotation` (`self.StaticMesh`))))
  (set `self.Timer` 0.0)
  (set `self.StartLerpAngle` _relativerotation_yaw))

(fn `SetLightPosition`
  (`parent.SetLightPosition`))

(fn `UserConstructionScript`
  (`parent.UserConstructionScript`))