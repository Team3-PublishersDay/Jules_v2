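; Light-interactable platform that rotates its mesh in repeating steps once it holds enough light from the Gauntlet, or when a connector triggers it.
; Tick waits between steps, lerps by a fixed rotation increment over a velocity-derived duration, and plays a sound once per step.
; EndAction is blocked mid-turn; stopping saves the step rotation as the next start.
; Level restart stops ticking and restores a start rotation depending on held light.
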(event `self.ReceiveBeginPlay`
  (`self.SetActorTickEnabled` self false)
  (`SceneComponent.K2_SetRelativeRotation` (`self.StaticMesh`) (`self.StartedRotation`) false false)
  (set `self.CachedStartedRotation` (`self.StartedRotation`))
  (`parent.ReceiveBeginPlay`))

(event `self.StartAction`
  (params (Gauntlet :type "/Game/Blueprints/InteractionSystem/Gauntlet/BP_Gauntlet Object Reference"))
  (`parent.StartAction` Gauntlet)
  (`self.HasRequiredLight`
    (:`HasRequiredLight`
      (`self.Perform`))))

(event `self.EndAction`
  (params (Gauntlet :type "/Game/Blueprints/InteractionSystem/Gauntlet/BP_Gauntlet Object Reference"))
  (if (`self.CanInteract`)
    (`parent.EndAction` Gauntlet)
    (`self.HasRequiredLight`
      (:`Doesen'tHaveRequiredLight`
        (`self.EndPerform`)))))

(event `self.ReceiveTick`
  (params (DeltaSeconds :type "Float (single-precision)"))
  (if (`self.CanPerform`)
    (bind _output_get (set `self.Timer` (`self.IncrementTimer` (`self.Timer`))))
    (if (>= _output_get (`self.TimeBeforeNextStep`))
      (set `self.CanInteract` false)
      (`self.Lerp` (`self.StartedLerpRotation`) (`self.EndedLerpRotation`))
      (`self.PlaySoundRotator`)
      (if (>= (`self.LerpTimer`) (`self.LerpDuration`))
        (`SceneComponent.K2_SetRelativeRotation` (`self.StaticMesh`) (`self.EndedLerpRotation`) false false)
        (`self.SetLerpData`)
        (set `self.CanPerform` false)))
    (else
      (`self.SetNextRotation`)
      (set `self.CanInteract` true)
      (set `self.CanPerform` true)
      (`self.Reset`))))

(event `PlaySoundRotator`
  ;[0 0 0] PlaySound
  (`/Engine/EditorBlueprintResources/StandardMacros.DoOnce` false :!label _label
    (:`Completed`
      (`GameplayStatics.PlaySoundAtLocation` (`self.RotatorSound`) (`self.K2_GetActorLocation` self) (struct) 1.0 1.0 0.0 null null null null))))

(event `/Game/Blueprints/InteractionSystem/LightInteract/Interface/BPI_Generator.StartConnector`
  (if (`self.IsIteractable`)
    (`self.HasRequiredLight`
      (:`Doesen'tHaveRequiredLight`
        _)))
  (`self.Perform`))

(event `Reset`
  ;[0 0 0] PlaySound
  (goto _label :!via `Reset`))

(event `/Game/Blueprints/InteractionSystem/LightInteract/Interface/BPI_Generator.EndConnector`
  (if (`self.IsIteractable`)
    (`self.HasRequiredLight`
      (:`Doesen'tHaveRequiredLight`
        _)))
  (`self.EndPerform`))

(fn `EndPerform`
  (`parent.EndPerform`)
  (`self.SetActorTickEnabled` self false)
  (if (> (`self.Timer`) (`self.TimeBeforeNextStep`))
    (`SceneComponent.K2_SetRelativeRotation` (`self.StaticMesh`) (`self.EndedLerpRotation`) false false)
    (set `self.StartedRotation` (`self.EndedLerpRotation`))
    (else
      (set `self.StartedRotation` (`self.StartedLerpRotation`))))
  (`self.SetLerpData`)
  (set `self.CanPerform` false))

(fn `GetLerpDuration`
  (returns (ReturnValue :type "Float (double-precision)"))
  (return (* (/ (`KismetMathLibrary.Abs` (`KismetMathLibrary.Vector_Distance` (`KismetMathLibrary.Conv_RotatorToVector` (`self.StartedRotation`)) (`KismetMathLibrary.Conv_RotatorToVector` (`self.EndedLerpRotation`)))) (`self.RotateVelocity`)) 100.0)))

(fn `IncrementTimer`
  (params (Time :type "Float (double-precision)"))
  (returns (ReturnValue :type "Float (double-precision)"))
  (return (+ (* (`GameplayStatics.GetWorldDeltaSeconds`) (`self.ElapsedTime`)) Time)))

(fn `Lerp`
  (params (A :type "Rotator Structure") (B :type "Rotator Structure"))
  (bind _output_get (set `self.LerpTimer` (`self.IncrementTimer` (`self.LerpTimer`))))
  (`SceneComponent.K2_SetRelativeRotation` (`self.StaticMesh`) (`KismetMathLibrary.RLerp` A B (/ _output_get (`self.LerpDuration`))) false false))

(fn `Perform`
  (`parent.Perform`)
  (set `self.CanPerform` true)
  (`self.SetLerpData`)
  (`self.SetInitRotation`)
  (set `self.LerpDuration` (`self.GetLerpDuration`))
  (`self.SetActorTickEnabled` self true))

(fn `RestartLevel`
  (`parent.RestartLevel`)
  (if (> (`self.AmmountOfLight`) 0)
    (`KismetArrayLibrary.Array_Clear` (`self.CurrentLights`))
    (set `self.CanPerform` false)
    (`SceneComponent.K2_SetRelativeRotation` (`self.StaticMesh`) (`self.StartedRotation`) false false)
    (`self.SetActorTickEnabled` self false)
    (else
      (set `self.CanPerform` false)
      (`SceneComponent.K2_SetRelativeRotation` (`self.StaticMesh`) (`self.CachedStartedRotation`) false false)
      (`self.SetActorTickEnabled` self false))))

(fn `SetInitRotation`
  (bind (_startedrotation_roll _startedrotation_pitch _startedrotation_yaw) (`KismetMathLibrary.BreakRotator` (`self.StartedRotation`)))
  (bind (_endedrotation_roll _endedrotation_pitch _endedrotation_yaw) (`KismetMathLibrary.BreakRotator` (`self.EndedRotation`)))
  (set `self.StartedLerpRotation` (`self.StartedRotation`))
  (set `self.EndedLerpRotation` (`KismetMathLibrary.MakeRotator` (+ _startedrotation_roll _endedrotation_roll) (+ _startedrotation_pitch _endedrotation_pitch) (+ _startedrotation_yaw _endedrotation_yaw)))
  (return))

(fn `SetLerpData`
  (set `self.Timer` 0.0)
  (set `self.LerpTimer` 0.0))

(fn `SetNextRotation`
  (bind (_startedlerprotation_roll _startedlerprotation_pitch _startedlerprotation_yaw) (`KismetMathLibrary.BreakRotator` (`self.StartedLerpRotation`)))
  (bind (_endedrotation_roll _endedrotation_pitch _endedrotation_yaw) (`KismetMathLibrary.BreakRotator` (`self.EndedRotation`)))
  (set `self.StartedLerpRotation` (`self.EndedLerpRotation`))
  (set `self.EndedLerpRotation` (`KismetMathLibrary.MakeRotator` (+ _startedlerprotation_roll _endedrotation_roll) (+ _startedlerprotation_pitch _endedrotation_pitch) (+ _startedlerprotation_yaw _endedrotation_yaw)))
  (return))

(fn `UserConstructionScript`
  (`parent.UserConstructionScript`))