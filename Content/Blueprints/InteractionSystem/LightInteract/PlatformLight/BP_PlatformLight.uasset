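; Light-interactable platform that moves its mesh along a spline, ping-ponging between the ends while active.
; Gauntlet actions drive it through a required-light threshold, and connector events can also start or stop it.
; On deactivation a DoOnce pauses it for a delay, then negative speed returns it to the spline start.
; Tick runs only from activation until it is home, and level restart clears its lights and reverses it.
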(event `self.ReceiveBeginPlay`
  (`self.SetActorTickEnabled` self false)
  (set `self.CachedSpeed` (`self.Spline Speed`))
  (`parent.ReceiveBeginPlay`))

(event `self.StartAction`
  (params (Gauntlet :type "/Game/Blueprints/InteractionSystem/Gauntlet/BP_Gauntlet Object Reference"))
  (`parent.StartAction` Gauntlet)
  (`self.HasRequiredLight`
    (:`Has Required Light`
      (`self.Perform`))))

(event `self.EndAction`
  (params (Gauntlet :type "/Game/Blueprints/InteractionSystem/Gauntlet/BP_Gauntlet Object Reference"))
  (`parent.EndAction` Gauntlet)
  (`self.HasRequiredLight`
    (:`Doesen't Have Required Light`
      (`self.EndPerform`))))

(event `self.ReceiveTick`
  (params (DeltaSeconds :type "Float (single-precision)"))
  (if (`self.CanPerform`)
    (set `self.Distance ` (`self.GetDistance` DeltaSeconds))
    (`self.PerformSpline`)
    (`self.GetLightSlot`)
    (`self.SetSpeedDirection`)
    (goto _label :!via `Reset`)
    (elif (<= (`self.Distance `) 0.0)
      (`self.SetActorTickEnabled` self false)
      (else
        (`|ExecutionSequence`
          (:`then_0`
            (`/Engine/EditorBlueprintResources/StandardMacros.DoOnce` false :!label _label
              (:`Completed`
                (set `self.CachedSpeed` (`self.Spline Speed`))
                (set `self.Spline Speed` 0.0)
                (`KismetSystemLibrary.Delay` (`self.DelayBeforeComeBack`))
                (set `self.Spline Speed` (`KismetMathLibrary.Abs` (`self.CachedSpeed`)))
                (set `self.Spline Speed` (* (`self.Spline Speed`) -1.0)))))
          (:`then_1`
            (set `self.Distance ` (`self.GetDistance` (`GameplayStatics.GetWorldDeltaSeconds`)))
            (`self.PerformSpline`)
            (`self.GetLightSlot`)
            (if (<= (`self.Distance `) 0.0)
              (goto _label :!via `Reset`))))))))

(event `/Game/Blueprints/InteractionSystem/LightInteract/Interface/BPI_Generator.StartConnector`
  (if (`self.IsIteractable`)
    (`self.HasRequiredLight`
      (:`Doesen't Have Required Light`
        _)))
  (`self.Perform`))

(event `/Game/Blueprints/InteractionSystem/LightInteract/Interface/BPI_Generator.EndConnector`
  (if (`self.IsIteractable`)
    (`self.HasRequiredLight`
      (:`Doesen't Have Required Light`
        _)))
  (`self.EndPerform`))

(fn `EndPerform`
  (`parent.EndPerform`)
  (set `self.CanPerform` false)
  (set `self.Spline Speed` (`KismetMathLibrary.Abs` (`self.CachedSpeed`)))
  (set `self.Spline Speed` (* (`self.Spline Speed`) -1.0)))

(fn `GetDistance`
  (params (TimeDeltaTime :type "Float (double-precision)"))
  (returns (Direction :type "Float (double-precision)"))
  (return (+ (* TimeDeltaTime (`self.Spline Speed`)) (`self.Distance `))))

(fn `Perform`
  (`parent.Perform`)
  (set `self.CanPerform` true)
  (set `self.Spline Speed` (`KismetMathLibrary.Abs` (`self.CachedSpeed`)))
  (`self.SetActorTickEnabled` self true))

(fn `PerformSpline`
  (`SceneComponent.K2_SetWorldTransform` (`self.StaticMesh`) (`KismetMathLibrary.MakeTransform` (.location (`SplineComponent.GetTransformAtDistanceAlongSpline` (`self.Spline`) (`self.Distance `) "World" false)) (`KismetMathLibrary.MakeRotator` 0.0) (`SceneComponent.RelativeScale3D` (`self.StaticMesh`))) false false))

(fn `RestartLevel`
  (`parent.RestartLevel`)
  (`KismetArrayLibrary.Array_Clear` (`self.CurrentLights`))
  (set `self.CanPerform` false)
  (set `self.Spline Speed` (`KismetMathLibrary.Abs` (`self.CachedSpeed`)))
  (set `self.Spline Speed` (* (`self.Spline Speed`) -1.0)))

(fn `SetSpeedDirection`
  (if (or (>= (`self.Distance `) (`SplineComponent.GetSplineLength` (`self.Spline`))) (<= (`self.Distance `) 0.0))
    (set `self.Spline Speed` (* (`self.Spline Speed`) -1.0))))

(fn `UserConstructionScript`
  (`parent.UserConstructionScript`))