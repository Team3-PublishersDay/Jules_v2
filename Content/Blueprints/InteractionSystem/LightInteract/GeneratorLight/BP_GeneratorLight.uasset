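; Light-powered generator interactable that switches on its connected actors while it holds enough light from the Gauntlet.
; Reaching the required light starts a looping-capable 2D sound, messages Connector actors through BPI_Generator and enables Tick for a timer.
; Dropping below the requirement stops it; timer expiry also returns the lights to their initial owners and blocks EndAction via CanInteract.
; Level restart clears the lights, ends connector messages and disables Tick.
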(event `self.ReceiveBeginPlay`
  (`self.SetActorTickEnabled` self false)
  (`parent.ReceiveBeginPlay`))

(event `self.StartAction`
  (params (Gauntlet :type "/Game/Blueprints/InteractionSystem/BP_Gauntlett Object Reference"))
  (`parent.StartAction` Gauntlet)
  (`self.HasRequiredLight`
    (:`HasRequiredLight`
      (`self.Perform`)
      (bind _returnvalue (`GameplayStatics.CreateSound2D` (`self.GeneratorSound`) 1.0 1.0 0.0 null))
      (`AudioComponent.Play` _returnvalue 0.0))))

(event `self.EndAction`
  (params (Gauntlet :type "/Game/Blueprints/InteractionSystem/BP_Gauntlett Object Reference"))
  (if (`self.CanInteract`)
    (`parent.EndAction` Gauntlet)
    (`self.HasRequiredLight`
      (:`Doesen'tHaveRequiredLight`
        (`self.EndPerform`)
        (`AudioComponent.Stop` (stale `self.StartAction` _returnvalue) :!label _label)
        (`self.PlaySounds` (`self.GeneratorEndSound`))))))

(event `self.ReceiveTick`
  (params (DeltaSeconds :type "Float (single-precision)"))
  (bind _output_get (set `self.Timer` (`self.IncrementTimer`)))
  (if (>= _output_get (`self.Duration`))
    (`self.PlaySounds` (`self.GeneratorEndSound`))
    (set `self.CanInteract` false)
    (for _array_element (`self.CurrentLights`)
      (`/Game/Blueprints/InteractionSystem/Light/BP_Lights.TurnBackToTheInitialOwner` _array_element _array_element))
    (for _array_element_2 (`self.Connector`)
      (if (`KismetSystemLibrary.DoesImplementInterface` _array_element_2 "/Game/Blueprints/InteractionSystem/LightInteract/Interface/BPI_Generator.BPI_Generator_C")
        (message `/Game/Blueprints/InteractionSystem/LightInteract/Interface/BPI_Generator.EndConnector` _array_element_2)))
    (`KismetArrayLibrary.Array_Clear` (`self.CurrentLights`))
    (`self.SetActorTickEnabled` self false)
    (goto _label)))

(fn `EndPerform`
  (`parent.EndPerform`)
  (if (`self.CanPerform`)
    (for _array_element (`self.Connector`)
      (if (`KismetSystemLibrary.DoesImplementInterface` _array_element "/Game/Blueprints/InteractionSystem/LightInteract/Interface/BPI_Generator.BPI_Generator_C")
        (message `/Game/Blueprints/InteractionSystem/LightInteract/Interface/BPI_Generator.EndConnector` _array_element)))
    (set `self.CanPerform` false)
    (`self.SetActorTickEnabled` self false)))

(fn `IncrementTimer`
  (returns (NewTimer :type "Float (double-precision)"))
  (return (+ (* (`GameplayStatics.GetWorldDeltaSeconds`) (`self.ElapsedTime`)) (`self.Timer`))))

(fn `Perform`
  (`parent.Perform`)
  (set `self.CanPerform` true)
  (set `self.CanInteract` true)
  (for _array_element (`self.Connector`)
    (if (`KismetSystemLibrary.DoesImplementInterface` _array_element "/Game/Blueprints/InteractionSystem/LightInteract/Interface/BPI_Generator.BPI_Generator_C")
      (message `/Game/Blueprints/InteractionSystem/LightInteract/Interface/BPI_Generator.StartConnector` _array_element)))
  (set `self.Timer` 0.0)
  (`self.SetActorTickEnabled` self true))

(fn `PlaySounds`
  (params (Sound :type "SoundBase Object Reference"))
  (`GameplayStatics.PlaySoundAtLocation` Sound (`SceneComponent.K2_GetComponentLocation` (`self.StaticMesh`)) (struct) 1.0 1.0 0.0 null null null null))

(fn `RestartLevel`
  (`parent.RestartLevel`)
  (`KismetArrayLibrary.Array_Clear` (`self.CurrentLights`))
  (for _array_element (`self.Connector`)
    (if (`KismetSystemLibrary.DoesImplementInterface` _array_element "/Game/Blueprints/InteractionSystem/LightInteract/Interface/BPI_Generator.BPI_Generator_C")
      (message `/Game/Blueprints/InteractionSystem/LightInteract/Interface/BPI_Generator.EndConnector` _array_element)))
  (set `self.CanPerform` false)
  (`self.SetActorTickEnabled` self false))

(fn `UserConstructionScript`
  (`parent.UserConstructionScript`))