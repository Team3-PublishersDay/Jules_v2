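; An altar light interactable that reports to a sequence puzzle when the Gauntlet interacts with it.
; If not already triggered, StartAction calls OnUpdateSequence with itself, runs the parent action, then ends it immediately.
; It can play a sequence sound at its location and briefly show a wrong-sequence material on its Sphere.
; The Sphere then switches to the material cached from StaticMesh at BeginPlay.
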(event `self.ReceiveBeginPlay`
  (`parent.ReceiveBeginPlay`)
  (set `self.InitialMaterial` (`PrimitiveComponent.GetMaterial` (`self.StaticMesh`) 0)))

(event `self.StartAction`
  (params (Gauntlet :type "/Game/Blueprints/InteractionSystem/Gauntlet/BP_Gauntlet Object Reference"))
  (if (not (`self.IsTriggered`))
    (`self.OnUpdateSequence` self)
    (`parent.StartAction` Gauntlet)
    (`self.EndAction` Gauntlet)))

(event `self.EndAction`
  (params (Gauntlet :type "/Game/Blueprints/InteractionSystem/Gauntlet/BP_Gauntlet Object Reference"))
  (`parent.EndAction` Gauntlet))

(event `/Game/Blueprints/InteractionSystem/LightInteract/Interface/BPI_Generator.StartConnector`)

(event `/Game/Blueprints/InteractionSystem/LightInteract/Interface/BPI_Generator.EndConnector`)

(event `SoundSequence`
  (params (Sound :type "SoundBase Object Reference"))
  (`GameplayStatics.PlaySoundAtLocation` Sound (`self.K2_GetActorLocation`) (struct) 1.0 1.0 0.0 null null null null))

(event `MaterialWrongSequenceAnimation`
  (params (WrongMaterial :type "MaterialInterface Object Reference") (Duration :type "Float (single-precision)"))
  (`self.SwitchMaterial` WrongMaterial)
  (`KismetSystemLibrary.Delay` Duration)
  (`self.SwitchMaterial` (`self.InitialMaterial`)))

(fn `SwitchMaterial`
  (params (Material :type "MaterialInterface Object Reference"))
  (`PrimitiveComponent.SetMaterial` (`self.Sphere`) 0 Material))

(fn `UserConstructionScript`
  (`parent.UserConstructionScript`))