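; BP_Lights is a light orb that moves between owners, such as light interactables, by reassigning ownership and attaching to the new owner.
; A timeline lerps its location and scale during transfers, notifying the Gauntlet at start and end.
; It binds to the GameMode's restart event, apparently to return to its initial owner's light list.
; Niagara trail effects can be toggled, and switch off on BeginPlay and when movement finishes.
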(event `self.ReceiveBeginPlay`
  (bind _asbp_game_mode (cast `/Game/Blueprints/BP_GameMode` (`GameplayStatics.GetGameMode`)))
  (add `/Game/Blueprints/BP_GameMode.OnRestartLevel` _asbp_game_mode (`|CreateDelegate` :!event `Restart`))
  (`self.DisableNiagara`))

(event `Inizialize`
  (params (InitOwner :type "/Game/Blueprints/InteractionSystem/BP_StoringLightBase Object Reference"))
  (set `self.InitialOwner` InitOwner))

(event `SetOwnerInteract`
  (params (Owner :type "/Game/Blueprints/InteractionSystem/BP_StoringLightBase Object Reference"))
  (`self.SetOwner` Owner)
  (`self.K2_AttachToActor` Owner "None" "KeepWorld" "KeepWorld" "KeepWorld"))

(event `TurnBackToTheInitialOwner`
  (params (Light :type "/Game/Blueprints/InteractionSystem/Light/BP_Lights Object Reference"))
  (bind _initialowner (`self.InitialOwner`))
  (`self.SetOwnerInteract` _initialowner)
  (`self.AddLight` Light)
  (bind _asbp_interact_light_base (cast `/Game/Blueprints/InteractionSystem/BP_InteractLightBase` _initialowner))
  (`/Game/Blueprints/InteractionSystem/BP_StoringLightBase.GetLightSlot` _asbp_interact_light_base))

(event `AddLight`
  (params (Light :type "/Game/Blueprints/InteractionSystem/Light/BP_Lights Object Reference"))
  (`KismetArrayLibrary.Array_Add` (`/Game/Blueprints/InteractionSystem/BP_StoringLightBase.CurrentLights` (`self.InitialOwner`)) Light))

(event `Restart`
  (if (not (== (`self.InitialOwner`) (`self.GetOwner` self)))
    (`self.TurnBackToTheInitialOwner` self)))

(event `LightAnimation`
  (params (Gauntlet :type "/Game/Blueprints/InteractionSystem/BP_Gauntlett Object Reference") (PositionA :type "Vector Structure") (PositionB :type "Vector Structure") (CurrentScale :type "Vector Structure") (NewScale :type "Vector Structure"))
  (`/Game/Blueprints/InteractionSystem/BP_Gauntlett.StartLightAnimation` Gauntlet)
  (bind (_direction _timer) (`Timeline|AnimationLight` :!via `PlayFromStart`)
    (:`Update`
      (`self.K2_SetActorTransform` (`KismetMathLibrary.MakeTransform` (`KismetMathLibrary.VLerp` PositionA PositionB _timer) (struct) (`KismetMathLibrary.VLerp` CurrentScale NewScale _timer))))
    (:`Finished`
      (`self.K2_SetActorTransform` (`KismetMathLibrary.MakeTransform` PositionB (struct) NewScale) false true)
      (`self.DisableNiagara`)
      (`/Game/Blueprints/InteractionSystem/BP_Gauntlett.SetPosition` Gauntlet)
      (`/Game/Blueprints/InteractionSystem/BP_Gauntlett.EndLightAnimation` Gauntlet))))

(event `EnabledNiagara`
  (`ActorComponent.Activate` (`self.NS_OrbTrail`) false)
  (`ActorComponent.Activate` (`self.Niagara1`) false))

(event `DisableNiagara`
  (`ActorComponent.Deactivate` (`self.NS_OrbTrail`))
  (`ActorComponent.Deactivate` (`self.Niagara1`)))

(fn `UserConstructionScript`)