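; Game mode Blueprint that manages the Enhanced Input mapping context for the first local player.
; BeginPlay adds the current context at top priority value zero, and SwapContext removes it, adds the supplied one and stores that as current.
; Helper functions wrap the player controller's input subsystem, though the remove helper passes no context to the subsystem call.
; GetGameData is an empty stub.
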(event `self.ReceiveBeginPlay`
  ;[1 1 1] ENABLED INPUT FOR PLAYER
  (`self.AddMappingContext` (`self.CurrentMappingContext`)))

(event `SwapContext`
  (params (Input :type "InputMappingContext Object Reference"))
  (`self.RemoveMappingContext` (`self.CurrentMappingContext`))
  (`self.AddMappingContext` Input)
  (set `self.CurrentMappingContext` Input))

(fn `AddMappingContext`
  (params (Input :type "InputMappingContext Object Reference"))
  (`EnhancedInputSubsystemInterface.AddMappingContext` (pcsubsystem `EnhancedInputLocalPlayerSubsystem` (`GameplayStatics.GetPlayerController` 0)) Input 0 (struct)))

(fn `GetGameData`
  (returns (SaveGame :type "Object Object Reference"))
  (return null))

(fn `RemoveMappingContext`
  (params (Input :type "InputMappingContext Object Reference"))
  (`EnhancedInputSubsystemInterface.RemoveMappingContext` (pcsubsystem `EnhancedInputLocalPlayerSubsystem` (`GameplayStatics.GetPlayerController` 0)) null (struct)))

(fn `UserConstructionScript`)