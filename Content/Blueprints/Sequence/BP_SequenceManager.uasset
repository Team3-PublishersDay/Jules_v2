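; BP_SequenceManager runs an ordered-activation puzzle built from altars.
; It records each altar reported through OnUpdateSequence with a trial material, then checks the order once the count matches the target Sequence.
; A correct order plays success material and sound and messages BPI_Generator targets, provided triggered actions exist.
; A wrong order plays failure feedback and clears progress; GameMode level restarts reset it without the sound.
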(event `self.ReceiveBeginPlay`
  (bind _sequence (`self.Sequence`))
  (bind _asbp_game_mode (cast `/Game/Blueprints/BP_GameMode` (`GameplayStatics.GetGameMode`)))
  (add `/Game/Blueprints/BP_GameMode.OnRestartLevel` _asbp_game_mode (`|CreateDelegate` :!event `RestartLevel`))
  (for (_ _array_index) _sequence
    (add `/Game/Blueprints/InteractionSystem/LightInteract/AltarLight/BP_AltarLightSequence.OnUpdateSequence` (`|GetArrayItem` _sequence _array_index) (`|CreateDelegate` :!event `UpdateSequence`)))
  (set `self.Index` (- (`KismetArrayLibrary.Array_Length` (`self.Sequence`)) 1)))

(event `RestartLevel`
  (`self.WrongSequence`))

(event `UpdateSequence`
  (params (Altar :type "/Game/Blueprints/InteractionSystem/LightInteract/AltarLight/BP_AltarLightSequence Object Reference"))
  (set `/Game/Blueprints/InteractionSystem/LightInteract/AltarLight/BP_AltarLightSequence.IsTriggered` true Altar)
  (`/Game/Blueprints/InteractionSystem/LightInteract/AltarLight/BP_AltarLightSequence.SwitchMaterial` Altar (`self.TrySequenceMaterial`))
  (if (< (`KismetArrayLibrary.Array_Length` (`self.MyListSequence`)) (`self.Index`))
    (`KismetArrayLibrary.Array_Add` (`self.MyListSequence`) Altar)
    (else
      (`KismetArrayLibrary.Array_Add` (`self.MyListSequence`) Altar)
      (`self.CheckSequence`))))

(fn `CheckSequence`
  (locals (IsRight :type Boolean))
  (for (_array_element _array_index) (`self.Sequence`)
    (if (== (`|GetArrayItem` (`self.MyListSequence`) _array_index) _array_element)
      (set `local.IsRight` true)
      (else
        (set `local.IsRight` false)
        (break))))
  (if (`local.IsRight`)
    (`self.TryPerform`)
    (else
      (`self.WrongSequence`)
      (`self.PlayWrongSequenceSound`))))

(fn `PlayWrongSequenceSound`
  (for _array_element (`self.Sequence`)
    (`/Game/Blueprints/InteractionSystem/LightInteract/AltarLight/BP_AltarLightSequence.SoundSequence` _array_element (`self.WrongSound`))))

(fn `TryPerform`
  (if (> (`KismetArrayLibrary.Array_Length` (`self.TriggeredAction`)) 0)
    (for _array_element (`self.MyListSequence`)
      (`/Game/Blueprints/InteractionSystem/LightInteract/AltarLight/BP_AltarLightSequence.SwitchMaterial` _array_element (`self.RightSequenceMaterial`))
      (`/Game/Blueprints/InteractionSystem/LightInteract/AltarLight/BP_AltarLightSequence.SoundSequence` _array_element (`self.RightSound`)))
    (for _array_element_2 (`self.TriggeredAction`)
      (if (`KismetSystemLibrary.DoesImplementInterface` _array_element_2 "/Game/Blueprints/InteractionSystem/LightInteract/Interface/BPI_Generator.BPI_Generator_C")
        (message `/Game/Blueprints/InteractionSystem/LightInteract/Interface/BPI_Generator.StartConnector` _array_element_2)))))

(fn `UserConstructionScript`)

(fn `WrongSequence`
  (for _array_element (`self.Sequence`)
    (set `/Game/Blueprints/InteractionSystem/LightInteract/AltarLight/BP_AltarLightSequence.IsTriggered` false _array_element)
    (`/Game/Blueprints/InteractionSystem/LightInteract/AltarLight/BP_AltarLightSequence.MaterialWrongSequenceAnimation` _array_element (`self.WrongSequenceMaterial`) (`self.DelayAfterNormalMaterial`)))
  (`KismetArrayLibrary.Array_Clear` (`self.MyListSequence`)))