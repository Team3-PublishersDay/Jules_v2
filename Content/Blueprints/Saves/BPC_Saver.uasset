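; BPC_Saver is an actor component that relays save and load calls to its owner and the owner's components through BPI_SaveableObject.
; On BeginPlay it caches the saveable owner, scans components for the interface (each match overwrites AllComponents, keeping only the last), and requests a load from the GameInstance.
; SaveAllData and LoadAllData pass data to the owner, then to the stored components if NeddedToBeSaved finds any.
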(event `self.ReceiveBeginPlay`
  (bind _returnvalue (`self.GetOwner`))
  (bind _asbpi_saveable_object (cast `/Game/Blueprints/Saves/BPI_SaveableObject` _returnvalue)
    (:`then`
      (set `self.Saveable Object` _asbpi_saveable_object))
    (:`CastFailed`
      _))
  (for _array_element (`Actor.K2_GetComponentsByClass` _returnvalue "/Script/Engine.ActorComponent")
    (if (`KismetSystemLibrary.DoesImplementInterface` _array_element "/Game/Blueprints/Saves/BPI_SaveableObject.BPI_SaveableObject_C")
      (set `self.AllComponents` (`|MakeArray` _array_element))))
  (message `/Game/Blueprints/Saves/BPI_Persistent.RequestLoad` (`GameplayStatics.GetGameInstance`) self))

(event `/Game/Blueprints/Saves/BPI_SaveManager.SaveAllData`
  (params (SaveData :type "/Game/Blueprints/Saves/BP_SaveGame1 Object Reference"))
  (`/Game/Blueprints/Saves/BPI_SaveableObject.SaveData` (`self.Saveable Object`) SaveData)
  (`self.NeddedToBeSaved`
    (:`true`
      (for _array_element (`self.AllComponents`)
        (message `/Game/Blueprints/Saves/BPI_SaveableObject.SaveData` _array_element SaveData)))))

(event `/Game/Blueprints/Saves/BPI_SaveManager.LoadAllData`
  (params (SaveGame :type "/Game/Blueprints/Saves/BP_SaveGame1 Object Reference"))
  (`/Game/Blueprints/Saves/BPI_SaveableObject.LoadData` (`self.Saveable Object`) SaveGame)
  (`self.NeddedToBeSaved`
    (:`true`
      (for _array_element (`self.AllComponents`)
        (message `/Game/Blueprints/Saves/BPI_SaveableObject.LoadData` _array_element SaveGame)))))