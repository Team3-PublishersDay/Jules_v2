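; Legacy game instance that owns the game's single save object and loads it synchronously on Init, creating a fresh one if no slot exists.
; Loading and saving run either sync or async, with an OnGameLoaded notification fired only when an existing save loads.
; SavePlayer writes player data into the save object before saving, and GetGameData exposes that object.
; Async saves show a lazily created, reused saving widget until completion.
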(event `self.ReceiveInit`
  (`self.LoadGameData` false))

(event `/Game/Blueprints/Saves/OldSaveSystem/BPI_SaveGame.LoadGameData`
  (params (Async :type Boolean))
  ;[1 1 1] LoadGame
  (bind _returnvalue (`GameplayStatics.DoesSaveGameExist` (`self.SlotGame`)))
  (if _returnvalue
    (if Async
      (bind _savegame (`AsyncActionHandleSaveGame.AsyncLoadGameFromSlot` (`self.SlotGame`))
        (:`Completed`
          (bind _asbp_oldsave_game (cast `/Game/Blueprints/Saves/OldSaveSystem/BP_OLDSaveGame` _savegame))
          (set `self.SaveGame` _asbp_oldsave_game)
          (`self.OnGameLoaded`)))
      (else
        (bind _returnvalue_2 (`GameplayStatics.LoadGameFromSlot` (`self.SlotGame`)))
        (bind _asbp_oldsave_game_2 (cast `/Game/Blueprints/Saves/OldSaveSystem/BP_OLDSaveGame` _returnvalue_2))
        (set `self.SaveGame` _asbp_oldsave_game_2)
        (`self.OnGameLoaded`)))
    (else
      (bind _returnvalue_3 (`GameplayStatics.CreateSaveGameObject` "/Game/Blueprints/Saves/OldSaveSystem/BP_OLDSaveGame.BP_OLDSaveGame_C"))
      (set `self.SaveGame` _returnvalue_3))))

(event `/Game/Blueprints/Saves/OldSaveSystem/BPI_SaveGame.SaveGameData`
  (params (Async :type Boolean))
  ;[1 1 1] SaveGame
  (if Async
    (`AsyncActionHandleSaveGame.AsyncSaveGameToSlot` (`self.SaveGame`) (`self.SlotGame`)
      (:`then`
        (`self.ShowSavingWidget`))
      (:`Completed`
        (`self.HideSavingWidget`)))
    (else
      (`GameplayStatics.SaveGameToSlot` (`self.SaveGame`) (`self.SlotGame`)))))

(event `/Game/Blueprints/Saves/OldSaveSystem/BPI_SaveGame.SavePlayer`
  (params (Async :type Boolean) (PlayerSafeData :type "/Game/Blueprints/Saves/PlayerSave/S_PlayerSave Structure"))
  (set `/Game/Blueprints/Saves/OldSaveSystem/BP_OLDSaveGame.PlayerSave` PlayerSafeData (`self.SaveGame`))
  (`self.SaveGameData` Async))

(event `ShowSavingWidget`
  (bind _savingwidget (`self.SavingWidget`)
    (:`then`
      (`Widget.SetVisibility` _savingwidget "Visible"))
    (:`else`
      (bind _returnvalue (`|CreateWidget` "/Game/Blueprints/Saves/W_SaveGame.W_SaveGame_C"))
      (bind _output_get (set `self.SavingWidget` _returnvalue))
      (`UserWidget.AddToViewport` _output_get 0))))

(event `HideSavingWidget`
  (bind _savingwidget (`self.SavingWidget`)
    (:`then`
      (`Widget.SetVisibility` _savingwidget "Hidden"))
    (:`else`)))

(fn `GetGameData`
  (returns (SaveGame :type "/Game/Blueprints/Saves/OldSaveSystem/BP_OLDSaveGame Object Reference"))
  (return (`self.SaveGame`)))