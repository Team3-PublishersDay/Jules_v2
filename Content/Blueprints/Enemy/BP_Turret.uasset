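; Enemy turret that shoots at the player and can be temporarily disabled with lights from the player's gauntlet.
; While active, PawnSensing turns the mesh toward a seen player and spawns a bullet from the Arrow after a fire-rate delay.
; TryStartAction takes the gauntlet's last light if more are required, attaches it and stops firing.
; A Tick-driven delay then returns all lights to their initial owner and reactivates the turret.
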(event `self.PawnSensing.OnSeePawn`
  (params (Pawn :type "Pawn Object Reference"))
  (bind (_returnvalue_location _returnvalue_rotation) (`KismetMathLibrary.BreakTransform` (`SceneComponent.K2_GetComponentToWorld` (`self.Arrow`))))
  (if (`self.CanPerform`)
    (cast `/Game/Blueprints/Player/BP_Player` Pawn)
    (`SceneComponent.K2_SetRelativeRotation` (`self.StaticMesh`) (`KismetMathLibrary.FindLookAtRotation` (`self.K2_GetActorLocation`) (`self.K2_GetActorLocation` Pawn)) false false)
    (`KismetSystemLibrary.Delay` (`self.FireRate`))
    (`|SpawnActorFromClass` "/Game/Blueprints/Enemy/BP_BulletBase1.BP_BulletBase1_C" (`KismetMathLibrary.MakeTransform` _returnvalue_location _returnvalue_rotation) "Undefined" "MultiplyWithRoot" null null)))

(event `/Game/Blueprints/InteractionSystem/LightInteract/Interface/BPI_LightsInteract.TryStartAction`
  (params (Gauntlet :type "/Game/Blueprints/InteractionSystem/Gauntlet/BP_Gauntlet Object Reference"))
  (`self.HasRequiredLight` (`self.RequiredLight`)
    (:`false`
      (`self.GetLight` Gauntlet)
      (`self.SetLightPosition`)
      (`self.SetLightOwner`)
      (set `self.CanPerform` false))))

(event `GetLight`
  (params (Gauntlet :type "/Game/Blueprints/InteractionSystem/Gauntlet/BP_Gauntlet Object Reference"))
  (bind _currentlights (`/Game/Blueprints/InteractionSystem/BP_StoringLightBase.CurrentLights` Gauntlet))
  (bind _returnvalue (`KismetArrayLibrary.Array_LastIndex` (`/Game/Blueprints/InteractionSystem/BP_StoringLightBase.CurrentLights` Gauntlet)))
  (`KismetArrayLibrary.Array_Add` (`self.CurrentLights`) (`|GetArrayItem` _currentlights _returnvalue))
  (`KismetArrayLibrary.Array_Remove` _currentlights _returnvalue))

(event `EndAction`
  (for _array_element (`self.CurrentLights`)
    (`/Game/Blueprints/InteractionSystem/Light/BP_Lights.TurnBackToTheInitialOwner` _array_element _array_element))
  (set `self.CanPerform` true)
  (`KismetArrayLibrary.Array_Clear` (`self.CurrentLights`)))

(event `self.ReceiveTick`
  (params (DeltaSeconds :type "Float (single-precision)"))
  (if (not (`self.CanPerform`))
    (`KismetSystemLibrary.Delay` (`self.DelayAfterStartAction`))
    (`self.EndAction`)))

(fn `IsInteractable`
  (returns (IsInteractable :type Boolean))
  (return false))

(fn `SetLightOwner`
  (bind _output (`|GetArrayItem` (`self.CurrentLights`) (`KismetArrayLibrary.Array_LastIndex` (`self.CurrentLights`))))
  (`self.SetOwner` _output self)
  (`self.K2_AttachToActor` _output self "None" "SnapToTarget" "KeepWorld" "KeepWorld" true))

(fn `SetLightPosition`
  ;[0.1656 0 1] Check for Lights
  (`self.HasRequiredLight` 0
    (:`true`
      ;[1 0.8394 0] For each light
      (for _array_element (`self.CurrentLights`)
        ;[1 0 0.3185] Set the position
        (`self.K2_SetActorLocation` _array_element (`SceneComponent.K2_GetComponentLocation` (`self.Scene`)) false true)))))

(fn `UserConstructionScript`)