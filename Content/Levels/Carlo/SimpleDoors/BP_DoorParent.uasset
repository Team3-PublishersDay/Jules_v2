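; BP_DoorParent is a door base Blueprint that swings its static mesh open and can be unlocked by a linked quest gate.
; BeginPlay sets the starting yaw and, if LinkedQuestGate is valid, binds its completion to Open.
; The OpenTime timeline lerps yaw between start and open angles, and Close reverses it.
; A DoOnce on the timeline update plays the door sound once per swing, resetting on finish.
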(event `self.ReceiveBeginPlay`
  (`SceneComponent.K2_SetRelativeRotation` (`self.StaticMesh`) (`KismetMathLibrary.MakeRotator` 0.0 0.0 (`self.StartZAngle`)) false false)
  (`/Engine/EditorBlueprintResources/StandardMacros.IsValid` (`self.Linked Quest Gate `)
    (:`Is Valid`
      (add `/Game/Blueprints/QuestSystem/BP_QuestBase.OnComplete` (`self.Linked Quest Gate `) (delegate `OpenGate`)))))

(event `OpenGate`
  (`self.Open`))

(event `Open`
  (bind (_direction _alpha) (`Timeline|OpenTime` :!via `PlayFromStart` :!label _label)
    (:`Update`
      (`|ExecutionSequence`
        (:`then_0`
          (`SceneComponent.K2_SetRelativeRotation` (`self.StaticMesh`) (`KismetMathLibrary.MakeRotator` 0.0 0.0 (`KismetMathLibrary.Lerp` (`self.StartZAngle`) (`self.OpenZAngle`) _alpha)) false false))
        (:`then_1`
          (`/Engine/EditorBlueprintResources/StandardMacros.DoOnce` false :!label _label_2
            (:`Completed`
              (`GameplayStatics.PlaySoundAtLocation` "/Game/Audio/Door/SC_Door_0a.SC_Door_0a" (`self.K2_GetActorLocation`) (struct) 1.0 1.0 0.0 null null null null))))))
    (:`Finished`
      (goto _label_2 :!via `Reset`))))

(event `Close`
  (goto _label :!via `Reverse`))

(fn `UserConstructionScript`)