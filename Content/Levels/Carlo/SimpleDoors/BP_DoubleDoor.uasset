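; BP_DoubleDoor is a two-panel door that swings open and closed around the yaw axis.
; BeginPlay zeroes both panel rotations and binds an event to the Trigger's Triggered notification.
; Open plays the OpenClose timeline from the start, lerping each panel from a shared start angle to its own open angle.
; Close reverses that timeline when IsOpen is true, though these graphs never set that flag.
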(event `self.ReceiveBeginPlay`
  (`SceneComponent.K2_SetRelativeRotation` (`self.Door1`) (`KismetMathLibrary.MakeRotator` 0.0) false false)
  (`SceneComponent.K2_SetRelativeRotation` (`self.Door2`) (`KismetMathLibrary.MakeRotator` 0.0) false false)
  (add `/Game/Levels/Carlo/BP_Trigger.Triggered` (`self.Trigger`) (`|CreateDelegate` :!event `Open`)))

(event `Open`
  (bind (_direction _alpha) (`Timeline|Open-Close` :!via `PlayFromStart` :!label _label)
    (:`Update`
      (`SceneComponent.K2_SetRelativeRotation` (`self.Door1`) (`KismetMathLibrary.MakeRotator` 0.0 0.0 (`KismetMathLibrary.Lerp` (`self.StartZAngle`) (`self.Door1-OpenZAngle`) _alpha)) false false)
      (`SceneComponent.K2_SetRelativeRotation` (`self.Door2`) (`KismetMathLibrary.MakeRotator` 0.0 0.0 (`KismetMathLibrary.Lerp` (`self.StartZAngle`) (`self.Door2-OpenZAngle`) _alpha)) false false))))

(event `Close`
  (if (`self.IsOpen`)
    (goto _label :!via `Reverse`)))

(fn `UserConstructionScript`)