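; Call button for the hub elevator, activated when an assigned Quest completes, or left inactive if none is bound.
; Activation swaps the button to an emissive material and sets it pressable.
; While the player is in the trigger and it is pressable, Tick centers the mouse and enables click events.
; Clicking sends the Elevator to floor 0; the click handler itself checks neither state, and click events are never disabled here.
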(event `self.ReceiveBeginPlay`
  (`/Engine/EditorBlueprintResources/StandardMacros.IsValid` (`self.Quest`)
    (:`Is Valid`
      (add `/Game/Blueprints/QuestSystem/BP_QuestBase.OnComplete` (`self.Quest`) (delegate `Activate`)))))

(event `self.ReceiveTick`
  (params (DeltaSeconds :type "Float (single-precision)"))
  (bind _returnvalue (`GameplayStatics.GetPlayerController` 0))
  (bind (_returnvalue_x _returnvalue_y) (`KismetMathLibrary.BreakVector2D` (`WidgetLayoutLibrary.GetViewportSize`)))
  (if (and (`self.PlayerIsOn`) (`self.CanBePressed`))
    (`PlayerController.SetMouseLocation` _returnvalue (`KismetMathLibrary.FTrunc` (/ _returnvalue_x 2.0)) (`KismetMathLibrary.FTrunc` (/ _returnvalue_y 2.0)))
    (set `PlayerController.bEnableClickEvents` true _returnvalue)))

(event `Activate`
  (`PrimitiveComponent.SetMaterial` (`self.Button`) 0 "/Game/Materials/MM_EmissiveLight2_Inst1.MM_EmissiveLight2_Inst1")
  (set `self.CanBePressed` true))

(event `self.PlayerTrigger.OnComponentBeginOverlap`
  (params (OverlappedComponent :type "PrimitiveComponent Object Reference") (OtherActor :type "Actor Object Reference") (OtherComp :type "PrimitiveComponent Object Reference") (OtherBodyIndex :type Integer) (bFromSweep :type Boolean) (SweepResult :type "HitResult Structure (by ref)"))
  (cast `/Game/Blueprints/Player/BP_Player` OtherActor)
  (set `self.PlayerIsOn` true))

(event `self.Button.OnClicked`
  (params (TouchedComponent :type "PrimitiveComponent Object Reference") (ButtonPressed :type "Key Structure"))
  (`/Game/Blueprints/Elevetor_System/BP_HubElevator.MoveTo` (`self.Elevator`) 0 false))

(event `self.PlayerTrigger.OnComponentEndOverlap`
  (params (OverlappedComponent :type "PrimitiveComponent Object Reference") (OtherActor :type "Actor Object Reference") (OtherComp :type "PrimitiveComponent Object Reference") (OtherBodyIndex :type Integer))
  (cast `/Game/Blueprints/Player/BP_Player` OtherActor)
  (set `self.PlayerIsOn` false))

(fn `UserConstructionScript`)