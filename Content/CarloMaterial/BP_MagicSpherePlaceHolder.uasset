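; Placeholder magic sphere pickup that bobs in place and can advance a linked quest.
; A fast looping timer from BeginPlay drives a sine-wave vertical offset on the Sphere component, instead of using Tick.
; Player overlap plays a sound and effect, destroys the actor, then calls CompletePart on QuestRef if valid.
; It also binds to the quest's OnComplete, apparently to destroy itself when the quest finishes.
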(event `self.Collision.OnComponentBeginOverlap`
  (params (OverlappedComponent :type "PrimitiveComponent Object Reference") (OtherActor :type "Actor Object Reference") (OtherComp :type "PrimitiveComponent Object Reference") (OtherBodyIndex :type Integer) (bFromSweep :type Boolean) (SweepResult :type "HitResult Structure (by ref)"))
  (cast `/Game/Blueprints/Player/BP_Player` OtherActor)
  (`self.PickUpSphere`)
  (bind _questref (`self.QuestRef`)
    (:`then`
      (`/Game/Blueprints/QuestSystem/BP_SubQuestPart.CompletePart` _questref))
    (:`else`)))

(event `PickUpSphere`
  (bind _returnvalue (`self.K2_GetActorLocation`))
  (`GameplayStatics.PlaySoundAtLocation` "/Game/Audio/Portals/SC_Portal_0a.SC_Portal_0a" _returnvalue (struct) 1.0 1.0 0.0 null null null null)
  (`NiagaraFunctionLibrary.SpawnSystemAtLocation` "/Game/3D/VFX/PickUp/MagicPIckUp/VFX_PickUp.VFX_PickUp" _returnvalue)
  (`self.K2_DestroyActor`))

(event `Destroy`
  (`self.K2_DestroyActor`))

(event `self.ReceiveBeginPlay`
  (`SceneComponent.K2_SetRelativeLocation` (`self.Sphere`) (`self.StartLocation`) false false)
  (`KismetSystemLibrary.K2_SetTimerDelegate` (`|CreateDelegate` :!event `FloatAnimation`) 0.01 true)
  (bind _questref (`self.QuestRef`)
    (:`then`
      (add `/Game/Blueprints/QuestSystem/BP_QuestBase.OnComplete` _questref (`|CreateDelegate` :!event `Destroy `)))
    (:`else`)))

(event `FloatAnimation`
  (bind (_startlocation_x _startlocation_y _returnvalue) (`self.Up/DownAnimation`))
  ;[0.4115 0.4115 0.4115 0.545] Magic Sphere Up/Down Animation
  (`SceneComponent.K2_SetRelativeLocation` (`self.Sphere`) (`KismetMathLibrary.MakeVector` _startlocation_x _startlocation_y _returnvalue) false false))

(fn `Up/DownAnimation`
  (returns (StartLocation_X :type "Float (double-precision)") (StartLocation_Y :type "Float (double-precision)") (ReturnValue :type "Float (double-precision)"))
  (bind (_startlocation_x _startlocation_y _startlocation_z) (`KismetMathLibrary.BreakVector` (`self.StartLocation`)))
  (return _startlocation_x _startlocation_y (+ _startlocation_z (* (`self.Distance`) (`KismetMathLibrary.DegSin` (* (`self.GetGameTimeSinceCreation`) (`self.AnimationSpeed`)))))))

(fn `UserConstructionScript`)